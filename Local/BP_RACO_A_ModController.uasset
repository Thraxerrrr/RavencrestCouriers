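; Mod controller for RACO bird courier messaging: merges the mod's data tables, loads saved inventory and spawns the tracking system on the server.
; Endpoints register here and supply destination lists.
; Sending moves courier and payload into a shared transit inventory and assigns a timed message record to the courier.
; Delivery grants XP, offloads items and returns the bird to the sender, falling back to the sender or deleting everything when endpoints are missing.
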(event EventBeginPlay
  (|CallParentFunction)
  (if (Networking|IsServer)
    (Utilities|FlowControl|Sequence
      (:then_0
        (bind _result (|LoadInventory (Class|PersistenceComponent|GetUniqueID (Variables|Default|GetPersistenceComponent)))
          (:OnSuccess
            (Class|LoadInventoryCallProxy|ProcessInventoryData self _result))))
      (:then_1
        (Utilities|FlowControl|Delay 3.0)
        ;[1 1 1 0.2] Spawn tracking system (Server)
        (bind _outactors (Actor|GetAllActorsOfClass (Variables|Default|GetRACOTrackingSystem)))
        (if (Utilities|Array|IsEmpty _outactors)
          (Game|SpawnActorfromClass (Variables|Default|GetRACOTrackingSystem) (Math|Conversions|ToTransform(Vector) "0, 0, 0") "Undefined" "OverrideRootScale" self 0))))))

(fn ConstructionScript)

(fn ModDataTableOperations
  (Class|ModController|MergeDataTables "/Game/UI/Data/DataTables/DT_UIModuleTable.DT_UIModuleTable" "/Game/Mods/RavencrestCouriers/DataTables/DT_RACO_UIModules.DT_RACO_UIModules")
  (Class|ModController|MergeDataTables "/Game/UI/Data/DataTables/DT_CraftingGUIPanelTable.DT_CraftingGUIPanelTable" "/Game/Mods/RavencrestCouriers/DataTables/DT_RACO_CraftingGUIPanels.DT_RACO_CraftingGUIPanels")
  (Class|ModController|MergeDataTables "/Game/Items/ItemTable.ItemTable" "/Game/Mods/RavencrestCouriers/DataTables/DT_RACO_ItemTable.DT_RACO_ItemTable")
  (Class|ModController|MergeDataTables "/Game/Items/Recipes/RecipesTable.RecipesTable" "/Game/Mods/RavencrestCouriers/DataTables/DT_RACO_Recipes.DT_RACO_Recipes")
  (Class|ModController|MergeDataTables "/Game/Items/Feats/FeatTable.FeatTable" "/Game/Mods/RavencrestCouriers/DataTables/DT_RACO_Feats.DT_RACO_Feats")
  (Class|ModController|MergeDataTables "/Game/Systems/Cheats/CustomConsoleCommandsDataTable.CustomConsoleCommandsDataTable" "/Game/Mods/RavencrestCouriers/DataTables/DT_RACO_Commands.DT_RACO_Commands")
  (Class|ModController|MergeDataTables "/Game/UI/Data/DataTables/DT_ConstructionSubClassData.DT_ConstructionSubClassData" "/Game/Mods/RavencrestCouriers/DataTables/DT_RACO_ConstructionSubClass.DT_RACO_ConstructionSubClass"))

(fn GetListOfDestinations
  (params (Exclusion :type Actor%20Component%20Object%20Reference))
  (bind _output_get (LocalVariables|SetlocalEndpoints (Variables|Messaging|GetmessagingEndpoints)))
  (Utilities|Array|RemoveItem _output_get Exclusion)
  (Class|BPRACOIMessagingEndpoint|SerializeDestination(Message) (LocalVariables|GetlocalEndpoints) (LocalVariables|GetlocalDestinations))
  (return (LocalVariables|GetlocalDestinations)))

(fn RegisterEndpoint
  (params (endpoint :type Actor%20Component%20Object%20Reference))
  (bind _endpoint (LocalVariables|Getendpoint)
    (:then
      (Utilities|Array|AddUnique (Variables|Messaging|GetmessagingEndpoints) _endpoint))
    (:else)))

(fn TryDeliverMessage
  (params (courier :type Game%20Item%20Object%20Reference))
  (bind (_inventory _slot) (CallFunction|GetInventoryandSlot courier))
  (bind _message (Class|BPRACOIBird|GetMessageinTransit(Message) courier))
  (bind _output_get (LocalVariables|Setmessage _message))
  (bind _endpoint (CallFunction|GetEndpointbyUID (.senderID (Utilities|Struct|BreakSTRUCT_RACO_MessageInFlight _output_get))))
  (LocalVariables|Setsender _endpoint)
  (bind _endpoint_2 (CallFunction|GetEndpointbyUID (.recipientID (Utilities|Struct|BreakSTRUCT_RACO_MessageInFlight _output_get))))
  (bind _output_get_2 (LocalVariables|Setrecipient _endpoint_2))
  (Utilities|IsValid _output_get_2
    (:Is%20Valid
      (Default|GiveBirdMessagingXP (Variables|Default|GetRACO_ExperienceSystem) courier :!label _label)
      (LocalVariables|SetoffloadInventory (Class|ItemInventory|GetInventorybyType (Components|GetOwner (LocalVariables|Getrecipient)) "PlaceableInventory"))
      (bind _array_element (Utilities|ForEachLoopFast (Utilities|Struct|BreakSTRUCT_RACO_MessageInFlight (LocalVariables|Getmessage)))
        (:LoopBody
          (Class|ItemInventory|MoveItem (Variables|Default|GetRACO_TransitInventory) _array_element (LocalVariables|GetoffloadInventory) -1 -1 true))
        (:Completed
          (bind _returnvalue (Components|GetOwner (LocalVariables|Getsender)))
          (bind _hasfreeslots (Class|BPRACOINest|HasFreeNestingSlots(Message) _returnvalue))
          (Class|ItemInventory|MoveItem _inventory _slot (Class|ItemInventory|GetInventorybyType _returnvalue (select _hasfreeslots "PetInventory" "PlaceableInventory")) -1 -1 true)
          (Class|BPRACOIBird|ClearDelivery(Message) courier)
          (bind _templateid (Class|BPRACOIBird|GetBirdTemplateID(Message) courier))
          (Class|BPRACOIMessagingEndpoint|PlayBirdSound(Message) (LocalVariables|Getrecipient) _templateid)
          (if (!= (LocalVariables|Getsender) (LocalVariables|Getrecipient))
            (Class|BPRACOIMessagingEndpoint|PlayBirdSound(Message) (LocalVariables|Getsender) _templateid)))))
    (:Is%20Not%20Valid
      (bind _sender (LocalVariables|Getsender)
        (:then
          (LocalVariables|Setrecipient _sender)
          (goto _label))
        (:else
          (bind _array_element_2 (Utilities|ForEachLoopFast (Utilities|Struct|BreakSTRUCT_RACO_MessageInFlight (LocalVariables|Getmessage)))
            (:LoopBody
              (Class|ItemInventory|DeleteItems (Variables|Default|GetRACO_TransitInventory) _array_element_2 "messageLost" -1))
            (:Completed
              (Class|ItemInventory|DeleteItems (Variables|Default|GetRACO_TransitInventory) (Class|ItemInventory|GetItemIndex (Variables|Default|GetRACO_TransitInventory) courier) "messageLost" -1))))))))

(fn TryMoveMessageIntoTransit
  (params (senderID :type String) (recipientID :type String) (courier :type Game%20Item%20Object%20Reference) (payload :type Array%20of%20Game%20Item%20Object%20References) (weightPct :type Float%20%28double-precision%29))
  (bind _raco_transitinventory (Variables|Default|GetRACO_TransitInventory))
  (bind (_inventory _slot) (CallFunction|GetInventoryandSlot courier))
  (Utilities|FlowControl|Sequence
    (:then_0
      ;[1 1 1 0.2] Can message be moved into transit?
      (if (== (Class|GameItem|GetOwnerInventory courier) (Variables|Default|GetRACO_TransitInventory))
        (return false "This courier is currently in transit and unavailable")))
    (:then_1
      (if (not (> (Class|ItemInventory|GetFreeSpaceCount (Variables|Default|GetRACO_TransitInventory)) (Utilities|Array|Length payload)))
        (return false "Air routes are congested, please try again later")))
    (:then_2
      ;[1 1 1 0.2] Move courier and payload into transit
      (Class|ItemInventory|MoveItem _inventory _slot (Variables|Default|GetRACO_TransitInventory) -1 -1 true)
      (bind _array_element (Utilities|ForEachLoopFast payload)
        (:LoopBody
          (bind _returnvalue (Class|ItemInventory|GetFirstFreeIndex _raco_transitinventory true))
          (bind _returnvalue_2 (Class|ItemInventory|MoveItem (.inventory (CallFunction|GetInventoryandSlot _array_element)) (.slot (CallFunction|GetInventoryandSlot _array_element)) _raco_transitinventory _returnvalue -1 true))
          (Utilities|Array|Add (LocalVariables|GetlocalTransitSlots) (Math|Integer|SelectInt _returnvalue -1 _returnvalue_2)))))
    (:then_3
      ;[1 1 1 0.2] Prepare message and assign it to courier
      (Utilities|Struct|SetmembersinSTRUCT_RACO_MessageInFlight (LocalVariables|GetlocalMessage) (Math|DateTime|UTCNow) senderID recipientID (LocalVariables|GetlocalTransitSlots))
      (bind _birdprofile (Class|BPRACOIBird|GetBirdProfile(Message) courier))
      (bind _structout (Utilities|Struct|SetmembersinSTRUCT_RACO_MessageInFlight (LocalVariables|GetlocalMessage) (CallFunction|CalculateTravelDuration (LocalVariables|GetlocalMessage) _birdprofile weightPct) true))
      (Class|BPRACOIBird|AssignDelivery(Message) courier _structout))
    (:then_4
      (return true ""))))

(fn UnregisterEndpoint
  (params (endpoint :type Actor%20Component%20Object%20Reference))
  (Utilities|Array|RemoveItem (Variables|Messaging|GetmessagingEndpoints) endpoint))