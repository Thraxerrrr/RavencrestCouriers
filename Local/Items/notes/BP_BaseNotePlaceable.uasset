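; Base Blueprint for placeable note items, linked to the RACO_Note document UI module.
; CanBePlaced runs the parent placement check but turns the "not vertical enough" failure into a success with an empty message.
; That error is detected by searching the failure text for "vertical" or "vertikal", so the bypass depends on message wording and language.
; All other placement results pass through unchanged.
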(event EventBeginPlay
  (|CallParentFunction))

(event Collision|EventActorBeginOverlap
  (params (OtherActor :type Actor%20Object%20Reference)))

(event EventTick
  (params (DeltaSeconds :type Float%20%28single-precision%29)))

(fn ConstructionScript
  (|CallParentFunction))

(fn CanbePlaced
  (params (AttachTo :type Buildable%20Base%20Object%20Reference) (InstanceIndex :type Integer))
  (bind (_failedmessage _returnvalue) (|CallParentFunction AttachTo InstanceIndex))
  ;[1 1 1] Ignore the error 'not vertical enough'
  (if (or (Utilities|String|Contains _failedmessage "vertical") (Utilities|String|Contains _failedmessage "vertikal"))
    (return "" "Success")
    (else
      (return _failedmessage _returnvalue))))

(fn GetDocUIModuleName
  (return "RACO_Note"))