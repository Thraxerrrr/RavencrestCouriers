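; BP_ParchmentScroll is a usable parchment item that opens a document UI for the player who uses it.
; On use, the server generates a DocumentID if the item lacks a valid one.
; If the user is player 0's character, that character's RACO actor component then requests the document UI with the item's reference.
; The item can always be used.
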(event EventOnUseItem
  (params (invokingCharacter :type Conan%20Character%20Object%20Reference) (ownerPlayer :type Conan%20Character%20Object%20Reference))
  (bind _returnvalue (Game|GetPlayerCharacter 0))
  (Utilities|FlowControl|Sequence
    (:then_0
      ;[1 1 1] On first use, generate a DocumentID
      (if (and (Networking|IsServer) (not (CallFunction|IsValidDocID (Variables|Default|GetdocumentID))))
        (Variables|Default|SetdocumentID (CallFunction|GenerateDocID))))
    (:then_1
      (if (== ownerPlayer _returnvalue)
        (bind _racoactorcomponent (CallFunction|GetRACOActorComp _returnvalue))
        (Default|RequestOpenDocumentUI _racoactorcomponent (CallFunction|GetGameItemRef self))))))

(fn CanUseItem
  (params (invokingCharacter :type Conan%20Character%20Object%20Reference))
  (return true))