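; BP_RACO_I_PaperObject is an interface-style contract for paper items that carry a document, with every function left as an empty stub.
; It declares actions to apply edits, copy an original and break a seal, the first two taking an instigator and returning success plus an info message.
; Accessors cover getting and setting the document and reporting paper type, item template ID and document UI module name.
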(fn TryApplyEdits
  (params (instigator :type Player%20Controller%20Object%20Reference) (document :type STRUCT%20RACO%20Document%20Structure))
  (return false ""))

(fn TryMakeCopy
  (params (original :type Object%20Object%20Reference) (instigator :type Player%20Controller%20Object%20Reference))
  (return false ""))

(fn TryBreakSeal
  (return false ""))

(fn GetDocUIModuleName
  (return "None"))

(fn GetPaperItemTemplateID
  (return 0))

(fn GetDocument
  (return ""))

(fn SetDocument
  (params (document :type STRUCT%20RACO%20Document%20Structure)))

(fn GetPaperType
  (return "None"))