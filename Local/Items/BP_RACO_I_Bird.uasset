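; BP_RACO_I_Bird is an interface for birds that can carry messages as deliveries.
; It declares getters for template ID and type, plus get and set pairs for the bird profile and detection config.
; Delivery functions assign a message, return the message in transit and clear the delivery.
; All functions are empty stubs, leaving the behavior to implementing classes.
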(fn GetBirdTemplateID
  (return 0))

(fn GetBirdType
  (return "None"))

(fn GetBirdProfile
  (return ""))

(fn SetBirdProfile
  (params (profile :type STRUCT%20RACO%20Bird%20Profile%20Structure))
  (return))

(fn AssignDelivery
  (params (message :type STRUCT%20RACO%20Message%20in%20Flight%20Structure)))

(fn GetMessageinTransit
  (return ""))

(fn ClearDelivery)

(fn GetDetectionConfig
  (return ""))

(fn SetDetectionConfig
  (params (newConfig :type STRUCT%20RACO%20Bird%20Detection%20Config%20Structure))
  (return false))