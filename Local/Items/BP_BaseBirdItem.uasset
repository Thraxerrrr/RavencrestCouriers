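; Base inventory item for a bird that has a profile and can act as a message courier.
; On data set, the server waits for the owner inventory to load, then creates a missing profile or reschedules a validated pending message at least 60 seconds out.
; Assigned deliveries run on a timer from submit time and travel duration, then ask the owner to deliver.
; Using the item opens the bird profile on the client.
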(event Custom|onInventoryDataLoaded
  (bind _entrustedmessage (Variables|Default|GetentrustedMessage))
  (bind (_submittimestamp _travelduration _validated) (Utilities|Struct|BreakSTRUCT_RACO_MessageInFlight _entrustedmessage))
  (EventDispatchers|UnbindEventfromOnSignalDataLoaded (stale EventSetData _inventory) (delegate Custom|onInventoryDataLoaded))
  (if (CallFunction|HasValidBirdID (Variables|Default|GetbirdProfile))
    (if _validated
      (CallFunction|ScheduleDelivery (Math|Float|Max(Float) (CallFunction|GetRemainingTime _submittimestamp _travelduration) 6e+01)))
    (else
      (CallFunction|InitNewBirdProfile (Variables|Default|GetbirdTypeID) (Variables|Default|GetbirdProfile))
      (Class|PersistenceComponent|SetDirty (Class|GameItem|GetOwnerInventory) true 5.0))))

(event Custom|TriggerStartPlacement
  (params (invokingCharacter :type Conan%20Character%20Object%20Reference) (ownerPlayer :type Conan%20Character%20Object%20Reference))
  ;[1 1 1 0.3] Use item
  (|CallParentFunction invokingCharacter ownerPlayer))

(event Custom|scheduleDelivery
  (params (timeToDelivery :type Float%20%28double-precision%29))
  ;[1 1 1 0.3] Courier
  (if (> timeToDelivery 0.99)
    (Utilities|Time|SetTimerbyEvent (delegate Custom|doDelivery) timeToDelivery)
    (else
      (Class|BPRACOIMessagingSystem|TryDeliverMessage(Message) (Class|GameItem|GetOwner) self))))

(event Custom|doDelivery
  ;[1 1 1 0.3] Courier
  (Class|BPRACOIMessagingSystem|TryDeliverMessage(Message) (Class|GameItem|GetOwner) self))

(event EventSetData
  (params (templateID :type Integer))
  (bind _entrustedmessage (Variables|Default|GetentrustedMessage))
  (bind (_submittimestamp _travelduration _validated) (Utilities|Struct|BreakSTRUCT_RACO_MessageInFlight _entrustedmessage))
  (|CallParentFunction templateID)
  (if (Networking|IsServer)
    (bind _inventory (Utilities|WaitforOwnerInventory))
    (if (Class|PersistenceComponent|IsDataDoneLoading _inventory)
      (if (CallFunction|HasValidBirdID (Variables|Default|GetbirdProfile))
        (if _validated
          (CallFunction|ScheduleDelivery (Math|Float|Max(Float) (CallFunction|GetRemainingTime _submittimestamp _travelduration) 6e+01)))
        (else
          (CallFunction|InitNewBirdProfile (Variables|Default|GetbirdTypeID) (Variables|Default|GetbirdProfile))
          (Class|PersistenceComponent|SetDirty (Class|GameItem|GetOwnerInventory) true 5.0)))
      (else
        (EventDispatchers|AssignOnSignalDataLoaded _inventory (delegate Custom|onInventoryDataLoaded))))))

(event EventAssignDelivery
  (params (message :type STRUCT%20RACO%20Message%20in%20Flight%20Structure))
  ;[1 1 1 0.3] Courier
  (bind _output_get (Variables|Default|SetentrustedMessage message))
  (CallFunction|ScheduleDelivery (CallFunction|GetRemainingTime (.submitTimestamp (Utilities|Struct|BreakSTRUCT_RACO_MessageInFlight _output_get)) (.travelDuration (Utilities|Struct|BreakSTRUCT_RACO_MessageInFlight _output_get))))
  (Class|PersistenceComponent|SetDirty (Class|GameItem|GetOwnerInventory) true 5.0))

(event EventClearDelivery
  ;[1 1 1 0.3] Courier
  (CallFunction|ClearMessage (Variables|Default|GetentrustedMessage))
  (Class|PersistenceComponent|SetDirty (Class|GameItem|GetOwnerInventory) true 5.0))

(event EventOnUseItem
  (params (invokingCharacter :type Conan%20Character%20Object%20Reference) (ownerPlayer :type Conan%20Character%20Object%20Reference))
  ;[1 1 1 0.3] Use item
  (if (not (Networking|IsServer))
    (Default|ClientOpenBirdProfile (CallFunction|GetBasePlayerCharRACO) self)))

(fn GetStatTexts
  (bind _birdtypeid (Variables|Default|GetbirdTypeID))
  (bind _birdtype (CallFunction|GetBirdTypebyID _birdtypeid))
  (bind _size (Utilities|Struct|BreakSTRUCT_RACO_BirdType _birdtype))
  (Utilities|FlowControl|Sequence
    (:then_0
      (if (not (Utilities|Array|IsEmpty _size))
        (LocalVariables|SetlocalStatOne (Utilities|Text|ToText(String) (Utilities|String|Append (CallFunction|CapitalizeFirstLetter _size) " bird")))))
    (:then_1
      (return (LocalVariables|GetlocalStatOne) "" ""))))

(fn GetBirdProfile
  (return (Variables|Default|GetbirdProfile)))

(fn GetBirdTemplateID
  (return (Variables|Default|GetTemplateID)))

(fn GetMessageinTransit
  (return (Variables|Default|GetentrustedMessage)))