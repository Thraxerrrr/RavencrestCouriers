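; Base inventory item for paper documents that can be read, edited, copied, sealed and placed, with stub type and UI module getters.
; On the server, SetData waits for owner inventory data to load, then initializes any document lacking a valid ID.
; A short timer on local use separates single tap (open document GUI or stop building) from double tap (notify placement, run parent use).
; Edits and copies are permission-checked and, like seal breaking, return success with a message.
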(event Custom|OnInventoryDataLoaded
  (EventDispatchers|UnbindallEventsfromOnSignalDataLoaded (stale EventSetData _returnvalue))
  (if (not (CallFunction|HasValidDocID (Variables|Default|Getdocument)))
    (CallFunction|InitNewDocument (Variables|Default|Getdocument))
    (Class|PersistenceComponent|SetDirty (Class|GameItem|GetOwnerInventory) true 5.0)))

(event Custom|OnSingleTap
  (Utilities|Time|ClearandInvalidateTimerbyHandle (Variables|Default|GetdelayedTimerHandle))
  (if (Variables|/Script/ConanSandbox.BuildSystemComponent|GetIsBuilding (Actor|GetComponentbyClass (stale EventOnUseItem invokingCharacter) "/Game/Systems/Building/BP_BuildSystem_v2.BP_BuildSystem_v2_C"))
    (Class|BuildSystemComponent|StopBuilding (Actor|GetComponentbyClass (stale EventOnUseItem invokingCharacter) "/Game/Systems/Building/BP_BuildSystem_v2.BP_BuildSystem_v2_C"))
    (else
      (Default|OpenDocumentGUIfromClient (CallFunction|GetCharacterRACO) (Utilities|GetGameItemRef)))))

(event EventSetData
  (params (templateID :type Integer))
  (|CallParentFunction templateID)
  (Utilities|FlowControl|Delay 0.0)
  (if (Networking|IsServer)
    (bind _returnvalue (Class|GameItem|GetOwnerInventory))
    (Utilities|IsValid _returnvalue
      (:Is%20Valid
        (if (Class|PersistenceComponent|IsDataDoneLoading _returnvalue)
          (if (not (CallFunction|HasValidDocID (Variables|Default|Getdocument)))
            (CallFunction|InitNewDocument (Variables|Default|Getdocument))
            (Class|PersistenceComponent|SetDirty (Class|GameItem|GetOwnerInventory) true 5.0))
          (else
            (EventDispatchers|AssignOnSignalDataLoaded _returnvalue (delegate Custom|OnInventoryDataLoaded))))))))

(event EventOnUseItem
  (params (invokingCharacter :type Conan%20Character%20Object%20Reference) (ownerPlayer :type Conan%20Character%20Object%20Reference))
  (Utilities|Or+Branch (Networking|IsDedicatedServer) (!= invokingCharacter (Game|GetPlayerCharacter 0))
    (:True
      (|CallParentFunction invokingCharacter ownerPlayer :!label _label))
    (:False
      (if (Utilities|Time|IsValidTimerHandle (Variables|Default|GetdelayedTimerHandle))
        (Utilities|Time|ClearandInvalidateTimerbyHandle (Variables|Default|GetdelayedTimerHandle))
        (Default|NotifyItemBeingPlaced (CallFunction|GetCharacterRACO) (Utilities|GetGameItemRef))
        (goto _label)
        (else
          (bind _returnvalue (Utilities|Time|SetTimerbyEvent (delegate Custom|OnSingleTap) 0.2))
          (Variables|Default|SetdelayedTimerHandle _returnvalue))))))

(fn CanUseItem
  (params (invokingCharacter :type Conan%20Character%20Object%20Reference))
  (return true))

(fn CanbeActivated
  (return false))

(fn GetShortDesc
  (return (Utilities|Text|ToText(String) (CallFunction|GetDocumentDescription (Variables|Default|Getdocument) true))))

(fn GetLongDesc
  (return (Utilities|Text|ToText(String) (CallFunction|GetDocumentDescription (Variables|Default|Getdocument) false))))

(fn GetDocUIModuleName
  (return "None"))

(fn GetDocument
  (return (Variables|Default|Getdocument)))

(fn GetDocumentType
  (return "None"))

(fn GetPaperItemTemplateID
  (return (Variables|Default|GetTemplateID)))

(fn SetDocument
  (params (document :type STRUCT%20RACO%20Document%20Structure))
  (Variables|Default|Setdocument document))

(fn TryApplyEdits
  (params (instigator :type Player%20Controller%20Object%20Reference) (document :type STRUCT%20RACO%20Document%20Structure))
  (if (CallFunction|CanEditDocument instigator self)
    (Variables|Default|Setdocument document)
    (return true "Document saved successfully!")
    (else
      (return false "You do not have permission to edit"))))

(fn TryBreakSeal
  (if (.sealed (Utilities|Struct|BreakSTRUCT_RACO_Document (Variables|Default|Getdocument)))
    (Utilities|Struct|SetmembersinSTRUCT_RACO_Document (Variables|Default|Getdocument) false)
    (return true "The seal has broken!")
    (else
      (return false "This document has no seal"))))

(fn TryMakeCopy
  (params (original :type Object%20Object%20Reference) (instigator :type Player%20Controller%20Object%20Reference))
  (Utilities|IsValid original
    (:Is%20Valid
      (if (CallFunction|CanCopyDocument instigator self)
        (bind _document (Class|BPRACOIDocument|GetDocument(Message) original))
        (bind _documentcopy (CallFunction|DuplicateDocument instigator _document))
        (Variables|Default|Setdocument _documentcopy)
        (return true "Document copied successfully!")
        (else
          (return false "You do not have permissions to copy"))))
    (:Is%20Not%20Valid
      (return false "The original document was not found"))))