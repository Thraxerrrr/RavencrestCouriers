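; Base placeable document actor that players can read and pick up, with stub functions for paper type, UI module, editing, seal breaking and copying.
; On placement it takes the document and item template ID from the placer's BP_RACO_AC_PlayerCharacter component and marks persistence dirty.
; Interacting opens the document GUI through that component.
; The radial menu adds a permission-checked Pick Up action that requests pickup through the component.
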(event Custom|OnPickupClicked
  (params (menuEntry :type Radial%20Menu%20Entry%20Object%20Reference))
  ;[1 1 1] Interaction wheel: add a custom PickUp action (that also remembers the document struct)
  (Default|ReqDocPickUp (CallFunction|GetPlayerCharacterAC) self))

(event EventInteractableMenu
  (params (RadialMenu :type Radial%20Menu%20Object%20Reference) (HitIndex :type Integer))
  ;[1 1 1] Interaction wheel: add a custom PickUp action (that also remembers the document struct)
  (|CallParentFunction RadialMenu HitIndex)
  (if (CallFunction|CanPickUpDocument (Pawn|GetControlledPawn (Widget|GetOwningPlayer RadialMenu)) self)
    (bind _returnvalue (Class|RadialMenu|AddItem RadialMenu "Pick Up" "Pick Up" "/Game/UI/Textures/GUIs/MainRadialMenu/T_MainRadialMenuIconPickup.T_MainRadialMenuIconPickup" "None" 0))
    (EventDispatchers|BindEventtoSignalClicked _returnvalue (delegate Custom|OnPickupClicked))))

(event EventOnPlaced
  (params (PlacedBy :type Conan%20Character%20Object%20Reference))
  (bind _returnvalue (Actor|GetComponentbyClass PlacedBy "/Game/Mods/RavencrestCouriers/System/BP_RACO_AC_PlayerCharacter.BP_RACO_AC_PlayerCharacter_C"))
  ;[1 1 1] After placement, retrieve document state from the RACO AC and apply to this Actor
  (Utilities|FlowControl|Sequence
    (:then_0
      (Variables|Default|Setdocument (Variables|/Game/Mods/RavencrestCouriers/System/BP_RACO_AC_PlayerCharacter.BP_RACO_AC_PlayerCharacter_C|GetdocBeingPlaced _returnvalue))
      (Variables|Default|SetdocItemTemplateID (Variables|/Game/Mods/RavencrestCouriers/System/BP_RACO_AC_PlayerCharacter.BP_RACO_AC_PlayerCharacter_C|GetdocTemplateID _returnvalue))
      (Class|PersistenceComponent|SetDirty (Variables|Default|GetConanBuildingPersistence) true 5.0))
    (:then_1
      (Default|NotifyItemPlacementDone _returnvalue))))

(event EventInteractableActivate
  (params (Component :type Primitive%20Component%20Object%20Reference) (Instigator :type Player%20Controller%20Object%20Reference) (HitIndex :type Integer) (TriggeredFromRadialWheel :type Boolean))
  ;[1 1 1] Default interaction: read the document
  (bind _document (CallFunction|GetDocument))
  (Default|OpenDocumentGUIfromServer (Actor|GetComponentbyClass (Pawn|GetControlledPawn Instigator) "/Game/Mods/RavencrestCouriers/System/BP_RACO_AC_PlayerCharacter.BP_RACO_AC_PlayerCharacter_C") self _document))

(fn ConstructionScript
  (|CallParentFunction))

(fn InteractableActivateDisabled
  (params (InteractingCharacter :type Conan%20Character%20Object%20Reference))
  (return false))

(fn GetDocUIModuleName
  (return "None"))

(fn GetDocument
  (return (Variables|Default|Getdocument)))

(fn GetPaperItemTemplateID
  (return (Variables|Default|GetdocItemTemplateID)))

(fn GetPaperType
  (return "None"))

(fn SetDocument
  (params (document :type STRUCT%20RACO%20Document%20Structure))
  (Variables|Default|Setdocument document))

(fn TryApplyEdits
  (params (instigator :type Player%20Controller%20Object%20Reference) (document :type STRUCT%20RACO%20Document%20Structure))
  (return false ""))

(fn TryBreakSeal
  (return false ""))

(fn TryMakeCopy
  (params (original :type Object%20Object%20Reference) (instigator :type Player%20Controller%20Object%20Reference))
  (return false ""))