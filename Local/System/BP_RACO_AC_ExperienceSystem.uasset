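; Actor component that awards experience and levels to RACO birds for messaging and for time elapsed.
; GiveBirdXP reads the bird's profile, adds XP, raises the level from GetVirtualBirdLevel when higher, grants one unspent point per level gained, then writes the profile back.
; Messaging and passive wrappers take their amounts from server settings, with passive XP prorating an hourly rate over a duration in seconds and truncating it.
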(fn GiveBirdXP
  (params (bird :type Object%20Object%20Reference) (amount :type Integer))
  (bind _birdprofile (Class|BPRACOIBird|GetBirdProfile(Message) bird))
  (LocalVariables|SetbirdProfile _birdprofile)
  (Utilities|FlowControl|Sequence
    (:then_0
      ;[1 1 1] Increase Experience Points
      (bind _structout (Utilities|Struct|SetmembersinSTRUCT_RACO_BirdProfile (LocalVariables|GetbirdProfile) (+ amount (Utilities|Struct|BreakSTRUCT_RACO_BirdProfile (LocalVariables|GetbirdProfile)))))
      (LocalVariables|SetbirdProfile _structout))
    (:then_1
      ;[1 1 1] Increase Level if applicable
      (bind _level (CallFunction|GetVirtualBirdLevel (.experience (Utilities|Struct|BreakSTRUCT_RACO_BirdProfile (LocalVariables|GetbirdProfile)))))
      (if (> _level (.level (Utilities|Struct|BreakSTRUCT_RACO_BirdProfile (LocalVariables|GetbirdProfile))))
        (bind _structout_2 (Utilities|Struct|SetmembersinSTRUCT_RACO_BirdProfile (LocalVariables|GetbirdProfile) _level (+ (- _level (.level (Utilities|Struct|BreakSTRUCT_RACO_BirdProfile (LocalVariables|GetbirdProfile)))) (.unspentPoints (Utilities|Struct|BreakSTRUCT_RACO_BirdProfile (LocalVariables|GetbirdProfile))))))
        (LocalVariables|SetbirdProfile _structout_2)))
    (:then_2
      (Class|BPRACOIBird|SetBirdProfile(Message) bird (LocalVariables|GetbirdProfile)))))

(fn GiveBirdMessagingXP
  (params (bird :type Object%20Object%20Reference))
  (CallFunction|GiveBirdXP bird (Default|GetBirdMessageXP (CallFunction|GetServerSettingsRACO))))

(fn GiveBirdPassiveXP
  (params (bird :type Object%20Object%20Reference) (Duration :type Float%20%28double-precision%29))
  (CallFunction|GiveBirdXP bird (Math|Float|Truncate (* (/ Duration 3.6e+03) (Default|GetBirdHourlyXP (CallFunction|GetServerSettingsRACO))))))