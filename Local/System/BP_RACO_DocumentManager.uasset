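; BP_RACO_DocumentManager is a persistent actor that stores RACO documents in a map keyed by document ID.
; On BeginPlay it gives itself a unique ID if it has none, so the persistence component can track it.
; Saving a document adds it to the map and marks persistence dirty with a short delay.
; Breaking a seal looks up a document, clears its Sealed flag and saves it back.
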(event EventBeginPlay
  (if (not (Class|DreamworldBlueprints|IsValidID (Class|PersistenceComponent|GetUniqueID (Variables|Default|GetActorPersistence))))
    (bind _returnvalue (Class|UniqueID|GenerateUniqueID))
    (Class|DreamworldBlueprints|SetUniqueID self _returnvalue)
    (Class|PersistenceComponent|SetDirty (Variables|Default|GetActorPersistence) true 5.0)))

(fn ConstructionScript)

(fn SaveDocument
  (params (documentID :type String) (document :type STRUCT%20RACO%20Document%20Structure))
  (Utilities|Map|Add (Variables|Default|GetdocumentStore) documentID document)
  (Class|PersistenceComponent|SetDirty (Variables|Default|GetActorPersistence) true 5.0))

(fn GetDocument
  (params (documentID :type String))
  (bind _documentstore (Variables|Default|GetdocumentStore))
  (bind (_value _returnvalue) (Utilities|Map|Find _documentstore documentID))
  (return _value _returnvalue))

(fn BreakDocumentSeal
  (params (documentID :type String))
  (bind (_document _documentfound) (CallFunction|GetDocument documentID))
  (if _documentfound
    (bind _structout (Utilities|Struct|SetmembersinSTRUCT_RACO_Document _document false))
    (CallFunction|SaveDocument documentID _structout)
    (return _structout)
    (else
      (return ""))))