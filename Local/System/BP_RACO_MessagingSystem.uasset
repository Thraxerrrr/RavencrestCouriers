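; Persistent messaging system that carries item payloads by courier bird between registered endpoint components.
; Accepted messages move bird and payload into a shared transit inventory and are queued with a travel time from base duration, bird speed and weight.
; A timer, started once server settings are available, polls the queue and delivers due messages, awarding bird XP.
; Missing recipients return messages to sender; if both endpoints are gone, the items are deleted.
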(event Custom|ProcessMessageQueueEvent
  ;[1 1 1] Start processing the message queue every X seconds
  (CallFunction|ProcessMessageQueue))

(event Custom|TryInit
  ;[1 1 1] Wait until SettingsSystem is available
  (Utilities|IsValid (CallFunction|GetSettingsSystem)
    (:Is%20Valid
      ;[1 1 1] Start processing the message queue every X seconds
      (Utilities|Time|SetTimerbyEvent (delegate Custom|ProcessMessageQueueEvent) (Math|Conversions|ToFloat(Integer) (.checkMessageFrequencySec (Utilities|Struct|BreakSTRUCT_RACO_ServerSettings (CallFunction|GetServerSettings)))) true))
    (:Is%20Not%20Valid
      (Utilities|Time|SetTimerbyEvent (delegate Custom|TryInit) 1.0))))

(event EventBeginPlay
  (Utilities|FlowControl|Sequence
    (:then_0
      ;[1 1 1] Register for DB persistence
      (if (not (Class|DreamworldBlueprints|IsValidID (Class|PersistenceComponent|GetUniqueID (Variables|Default|GetConanBuildingPersistence))))
        (bind _returnvalue (Class|UniqueID|GenerateUniqueID))
        (Class|DreamworldBlueprints|SetUniqueID self _returnvalue)
        (Class|PersistenceComponent|SetDirty (Variables|Default|GetConanBuildingPersistence) true 5.0)))
    (:then_1
      ;[1 1 1] Wait until SettingsSystem is available
      (Utilities|Time|SetTimerbyEvent (delegate Custom|TryInit) 1.0))))

(fn ConstructionScript)

(fn MoveMessageIntoTransit
  (params (senderID :type String) (receiverID :type String) (courier :type Game%20Item%20Object%20Reference) (payload :type Array%20of%20Game%20Item%20Object%20References) (weightPct :type Float%20%28double-precision%29))
  (Utilities|FlowControl|Sequence
    (:then_0
      ;[1 1 1] Message Validation
      (if (== (Class|GameItem|GetOwnerInventory courier) (Variables|Default|GetTransitItemInventory))
        (return false "The bird is currently in transit and unavailable!")))
    (:then_1
      (bind _hasfree (CallFunction|TransitHasSlotsFree (+ (Utilities|Array|Length payload) 1)))
      (if (not _hasfree)
        (return false "Message system congested, please try again later")))
    (:then_2
      ;[1 1 1] Move payload into transit
      (bind _transitslot (CallFunction|MoveItemtoTransit courier))
      (Utilities|Array|Add (LocalVariables|GettransitSlots) _transitslot)
      (for _array_element payload
        (bind _transitslot_2 (CallFunction|MoveItemtoTransit _array_element))
        (Utilities|Array|Add (LocalVariables|GettransitSlots) _transitslot_2)))
    (:then_3
      ;[1 1 1] Prepare a MessageRequest struct
      (Utilities|Struct|SetmembersinSTRUCT_RACO_MessageInFlight (LocalVariables|GetmessageReq) (Math|DateTime|Now) senderID receiverID (Variables|/Script/ConanSandbox.GameItem|GetTemplateID courier) (LocalVariables|GettransitSlots))
      (bind _birdprofile (Class|BPRACOICourier|GetBirdProfile(Message) courier))
      (bind _travelduration (CallFunction|CalculateTravelDuration (LocalVariables|GetmessageReq) _birdprofile weightPct))
      (Utilities|Struct|SetmembersinSTRUCT_RACO_MessageInFlight (LocalVariables|GetmessageReq) _travelduration))
    (:then_4
      ;[1 1 1] Register the message in the queue
      (Utilities|Array|Add (Variables|Default|GetmessagesInFlight) (LocalVariables|GetmessageReq))
      (Class|PersistenceComponent|SetDirty (Variables|Default|GetConanBuildingPersistence) true 5.0))
    (:then_5
      (return true ""))))

(fn ProcessMessageQueue
  (if (Utilities|Array|IsNotEmpty (Variables|Default|GetmessagesInFlight))
    (bind (_arrayindex _arrayelement) (Utilities|Array|ReverseforEachLoop (Variables|Default|GetmessagesInFlight))
      (:LoopBody
        (if (CallFunction|HasTimePassed (.submitTimestamp (Utilities|Struct|BreakSTRUCT_RACO_MessageInFlight _arrayelement)) (.travelDuration (Utilities|Struct|BreakSTRUCT_RACO_MessageInFlight _arrayelement)))
          (CallFunction|DeliverMessageNow _arrayelement)
          (Utilities|Array|RemoveIndex (Variables|Default|GetmessagesInFlight) _arrayindex)
          (Class|PersistenceComponent|SetDirty (Variables|Default|GetConanBuildingPersistence) true 5.0))))))

(fn DeliverMessageNow
  (params (message :type STRUCT%20RACO%20Message%20in%20Flight%20Structure))
  (bind (_senderid _recipientid) (Utilities|Struct|BreakSTRUCT_RACO_MessageInFlight message))
  (bind _endpoint (CallFunction|GetEndpointbyUID _senderid))
  (LocalVariables|Setsender _endpoint)
  (bind _endpoint_2 (CallFunction|GetEndpointbyUID _recipientid))
  (LocalVariables|Setreceiver _endpoint_2)
  (Utilities|FlowControl|Sequence
    (:then_0
      (bind _asbp_base_bird_item (Utilities|Casting|CastToBP_BaseBirdItem (Class|ItemInventory|GetItem (Variables|Default|GetTransitItemInventory) (Utilities|Array|Get(acopy) (Utilities|Struct|BreakSTRUCT_RACO_MessageInFlight message)))))
      (Default|GiveBirdMessagingXP (CallFunction|GetExperienceSystem) _asbp_base_bird_item))
    (:then_1
      (Utilities|IsValid (LocalVariables|Getreceiver)
        (:Is%20Valid
          (Default|DoReceiveMessage (LocalVariables|Getreceiver) message :!label _label)
          (Default|HandleMessageDeliveredNotification (LocalVariables|Getsender) message))
        (:Is%20Not%20Valid
          ;[1 1 1] Return to sender
          (Utilities|IsValid (LocalVariables|Getsender)
            (:Is%20Valid
              (LocalVariables|Setreceiver (LocalVariables|Getsender))
              (goto _label))
            (:Is%20Not%20Valid
              (CallFunction|DestroyMessage message))))))))

(fn CalculateTravelDuration
  (params (message :type STRUCT%20RACO%20Message%20in%20Flight%20Structure) (carrierProfile :type STRUCT%20RACO%20Bird%20Profile%20Structure) (weightPct :type Float%20%28double-precision%29))
  (if (<= weightPct 0.5)
    _
    (elif (<= weightPct 0.75)
      (LocalVariables|SetweightFactor 1.5)
      (else
        (LocalVariables|SetweightFactor 2.0))))
  (return (Math|Float|Truncate (* (/ (Math|Conversions|ToFloat(Integer) (Utilities|Struct|BreakSTRUCT_RACO_ServerSettings (CallFunction|GetServerSettings))) (CallFunction|CalcBirdTravelSpeed carrierProfile)) (LocalVariables|GetweightFactor)))))

(fn TransitHasSlotsFree
  (params (freeSlotCount :type Integer))
  (bind _transititeminventory (Variables|Default|GetTransitItemInventory))
  (return (<= freeSlotCount (- (Variables|/Script/ConanSandbox.ItemInventory|GetMaxItemCount _transititeminventory) (Class|ItemInventory|GetPopulatedItemCount _transititeminventory 0 -1)))))

(fn GetEndpointbyUID
  (params (uniqueID :type String))
  (bind _actor (Class|BaseGameModeInterface|GetActorbyUniqueIDInterface(Message) (Game|GetGameMode) (Class|UniqueID|MakeUID uniqueID)))
  (return (Actor|GetComponentbyClass _actor "/Game/Mods/RavencrestCouriers/System/BP_RACO_MessagingEndpoint_AC.BP_RACO_MessagingEndpoint_AC_C")))

(fn DestroyMessage
  (params (message :type STRUCT%20RACO%20Message%20in%20Flight%20Structure))
  (bind _array_element (Utilities|ForEachLoopFast (Utilities|Struct|BreakSTRUCT_RACO_MessageInFlight message))
    (:LoopBody
      (Class|ItemInventory|DeleteItems (Variables|Default|GetTransitItemInventory) _array_element "messageLost" -1))))

(fn GetListOfDestinations
  (params (Exclusion :type Actor%20Component%20Object%20Reference))
  (bind _output_get (LocalVariables|SetlocalEndpoints (Variables|Default|Getendpoints)))
  (Utilities|Array|RemoveItem _output_get Exclusion)
  (Class|BPRACOIMessagingEndpoint|SerializeDestination(Message) (LocalVariables|GetlocalEndpoints) (LocalVariables|GetlocalDestinations))
  (return (LocalVariables|GetlocalDestinations)))

(fn MoveItemfromTransit
  (params (transitSlot :type Integer) (targetInventory :type Item%20Inventory%20Object%20Reference))
  (if (>= transitSlot 0)
    (bind _returnvalue (Class|ItemInventory|MoveItem (Variables|Default|GetTransitItemInventory) transitSlot targetInventory -1 -1 true))
    (return _returnvalue)
    (else
      (return false))))

(fn MoveItemtoTransit
  (params (Item :type Game%20Item%20Object%20Reference))
  (bind _returnvalue (Class|GameItem|GetOwnerInventory Item))
  (bind _output_get (LocalVariables|SetlocalSlot (Class|ItemInventory|GetFirstFreeIndex (Variables|Default|GetTransitItemInventory) false)))
  (if (>= _output_get 0)
    (bind _returnvalue_2 (Class|ItemInventory|MoveItem _returnvalue (Class|ItemInventory|GetItemIndex _returnvalue Item) (Variables|Default|GetTransitItemInventory) (LocalVariables|GetlocalSlot) -1 false))
    (if _returnvalue_2
      (return (LocalVariables|GetlocalSlot))
      (else
        (return -1)))
    (else
      (return -1))))

(fn RegisterEndpoint
  (params (endpoint :type Actor%20Component%20Object%20Reference))
  (Utilities|Array|AddUnique (Variables|Default|Getendpoints) endpoint))

(fn UnregisterEndpoint
  (params (endpoint :type Actor%20Component%20Object%20Reference))
  (Utilities|Array|RemoveItem (Variables|Default|Getendpoints) endpoint))