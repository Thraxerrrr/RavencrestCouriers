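; Actor component that makes a Conan Exiles buildable an endpoint in the RACO mod's bird-courier messaging system, registering with the mod controller on the server.
; It lists itself as a destination when receiving is enabled and moves player items into its placeable inventory.
; Sending validates the nested bird, recipient, item locations and carry weight, then hands the message to the controller for transit and multicasts a bird sound.
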(event Custom|multicastPlayBirdSound
  (params (courierID :type Integer))
  (if (not (Networking|IsDedicatedServer))
    (bind _birdtype (CallFunction|GetBirdTypefromTemplateID courierID))
    (CallFunction|PlayBirdSound (Variables|Default|GetaudioComponent) _birdtype)))

(event EventPlayBirdSound
  (params (templateID :type Integer))
  (CallFunction|MulticastPlayBirdSound templateID))

(event EventEndPlay
  (params (EndPlayReason :type EEndPlayReason%20Enum :default "Destroyed"))
  ;[1 1 1 0.2] Register/unregister this messaging endpoint in the messaging system
  (if (Networking|IsServer)
    (if (not (CallFunction|IsABrush (Components|GetOwner)))
      (Class|BPRACOIMessagingSystem|UnregisterEndpoint(Message) (CallFunction|GetModControllerRACO) self))))

(event EventBeginPlay
  ;[1 1 1 0.2] Register/unregister this messaging endpoint in the messaging system
  (if (Networking|IsServer)
    (if (not (CallFunction|IsABrush (Components|GetOwner)))
      (Class|BPRACOIMessagingSystem|RegisterEndpoint(Message) (CallFunction|GetModControllerRACO) self))))

(fn GetDisplayName
  (bind _returnvalue (Components|GetOwner))
  (bind _asbuildable_base (Utilities|Casting|CastToBuildableBase _returnvalue))
  (bind _returnvalue_2 (Class|BuildableBase|GetOwnerName _asbuildable_base))
  (return (Utilities|String|Append (Utilities|String|ToString(Text) _returnvalue_2) " (" (Utilities|String|ToString(Text) (Class|BuildableBase|GetBuildableName _asbuildable_base false)) ")")))

(fn GetUniqueID
  (return (Class|DreamworldBlueprints|ToString(UniqueID) (Class|UniqueID|GetActorUID (Components|GetOwner)))))

(fn CanDepositItems
  (params (playerCharacter :type Actor%20Object%20Reference) (items :type Array%20of%20Game%20Item%20Object%20References))
  (Utilities|FlowControl|Sequence
    (:then_0
      (if (Utilities|Array|IsEmpty items)
        (return false "")))
    (:then_1
      (bind _playercharacter (LocalVariables|GetplayerCharacter)
        (:then
          (LocalVariables|SetacceptedInventories (Utilities|Array|MakeArray (Class|ItemInventory|GetInventorybyType _playercharacter "Backpack") (Class|ItemInventory|GetInventorybyType _playercharacter "ShortcutBar")))
          (bind _array_element (Utilities|ForEachLoopFast items)
            (:LoopBody
              (Utilities|IsValid _array_element
                (:Is%20Valid
                  (if (not (Utilities|Array|ContainsItem (LocalVariables|GetacceptedInventories) (Class|GameItem|GetOwnerInventory _array_element)))
                    (return false "Some items could not be found in inventory")))
                (:Is%20Not%20Valid
                  (return false ""))))))
        (:else
          (return false ""))))
    (:then_2
      (if (> (Utilities|Array|Length items) (Class|ItemInventory|GetFreeSpaceCount (Utilities|GetOwnerInventory "PlaceableInventory")))
        (return false "Not enough space to deposit everything")))
    (:then_3
      (return true ""))))

(fn GetCanReceive
  (return (Variables|Default|GetcanReceive)))

(fn SerializeDestination
  (params (destinations :type Array%20of%20Strings))
  (if (Variables|Default|GetcanReceive)
    (bind _name (CallFunction|GetDisplayName))
    (Utilities|Array|Add destinations (CallFunction|MakeEndpointString _name (CallFunction|GetUniqueID)))))

(fn SetCanReceive
  (params (canReceiveMessages :type Boolean))
  (Variables|Default|SetcanReceive canReceiveMessages)
  (Class|PersistenceComponent|SetDirty (Actor|GetComponentbyClass (Components|GetOwner) "/Script/ConanSandbox.ConanBuildingPersistenceComponent") true 5.0))

(fn TryDepositItems
  (params (playerCharacter :type Actor%20Object%20Reference) (items :type Array%20of%20Game%20Item%20Object%20References))
  (bind (_success _infomessage) (CallFunction|CanDepositItems playerCharacter items))
  (if _success
    (LocalVariables|SetlocalInventory (Utilities|GetOwnerInventory "PlaceableInventory"))
    (bind _array_element (Utilities|ForEachLoopFast items)
      (:LoopBody
        (Class|ItemInventory|MoveItem (.inventory (CallFunction|GetInventoryandSlot _array_element)) (.slot (CallFunction|GetInventoryandSlot _array_element)) (LocalVariables|GetlocalInventory) -1 -1 false))
      (:Completed
        (return true "")))
    (else
      (return false _infomessage))))

(fn TrySendMessage
  (params (playerCharacter :type Conan%20Character%20Object%20Reference) (courier :type Game%20Item%20Object%20Reference) (payload :type Array%20of%20Game%20Item%20Object%20References) (recipientID :type String))
  (bind (_success _infomessage _pctweight) (CallFunction|ValidateMessage playerCharacter courier payload recipientID))
  (if _success
    (bind (_success_2 _infomessage_2) (Class|BPRACOIMessagingSystem|TryMoveMessageIntoTransit(Message) (CallFunction|GetModControllerRACO) (CallFunction|GetUniqueID) recipientID courier payload _pctweight))
    (Utilities|FlowControl|Sequence
      (:then_0
        (if _success_2
          (bind _templateid (Class|BPRACOIBird|GetBirdTemplateID(Message) courier))
          (CallFunction|MulticastPlayBirdSound _templateid)))
      (:then_1
        (return _success_2 _infomessage_2)))
    (else
      (return false _infomessage))))

(fn ValidateMessage
  (params (playerCharacter :type Conan%20Character%20Object%20Reference) (courier :type Game%20Item%20Object%20Reference) (payload :type Array%20of%20Game%20Item%20Object%20References) (recipientID :type String))
  (Utilities|FlowControl|Sequence
    (:then_0
      (bind _courier (LocalVariables|Getcourier)
        (:then
          (if (not (CallFunction|IsBird _courier))
            (return false "Only nested birds can be couriers" 0.0)))
        (:else
          (if (Utilities|Array|IsEmpty payload)
            (return false "" 0.0)
            (else
              (return false "The message needs a courier" 0.0))))))
    (:then_1
      (bind _population (Class|BPRACOINest|GetNestPopulation(Message) (Components|GetOwner)))
      (if (not (Utilities|Array|ContainsItem _population courier))
        (return false "The courier is not nested" 0.0)))
    (:then_2
      (if (Class|DreamworldBlueprints|IsValidID (Class|UniqueID|MakeUID recipientID))
        (if (Utilities|Array|IsEmpty payload)
          (return true "" 0.0))
        (else
          (return false "The courier needs a valid destination" 0.0))))
    (:then_3
      (bind _playercharacter (LocalVariables|GetplayerCharacter)
        (:then
          (bind _returnvalue (Class|ConanCharacter|GetShortcutBarInventory _playercharacter))
          (LocalVariables|SetacceptedInventories (Utilities|Array|MakeArray (Utilities|GetOwnerInventory "PetInventory") (Utilities|GetOwnerInventory "PlaceableInventory") (Class|ConanCharacter|GetBackpackInventory playerCharacter) _returnvalue))
          (bind _array_element (Utilities|ForEachLoopFast payload)
            (:LoopBody
              (if (not (Utilities|Array|ContainsItem (LocalVariables|GetacceptedInventories) (Class|GameItem|GetOwnerInventory _array_element)))
                (return false "Some items could not be found in inventory" 0.0)))))
        (:else
          (return false "" 0.0))))
    (:then_4
      (if (Utilities|Array|ContainsItem payload courier)
        (return false "The courier cannot be part of the items" 0.0)))
    (:then_5
      (bind _birdprofile (Class|BPRACOIBird|GetBirdProfile(Message) courier))
      (bind _output_get (LocalVariables|SetlocalPctWeight (/ (CallFunction|GetTotalItemsWeight payload) (CallFunction|GetBirdCarryWeight _birdprofile))))
      (if (not (>= 1.0 _output_get))
        (return false "Message too heavy for this courier" 0.0)))
    (:then_6
      (return true "" (LocalVariables|GetlocalPctWeight)))))