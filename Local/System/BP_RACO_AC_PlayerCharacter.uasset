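; Player character component for the RACO mod, handling courier bird, messaging and document interactions between client UI and server in Conan.
; Req events resolve object refs and act through messages, answering through client callbacks that fire one-shot dispatchers.
; Documents sync to clients with sealed text redacted and optional truncation.
; Equipped birds replicate a profile that drives an animated shoulder mesh, earn passive XP on unequip and enable timer-driven tracking.
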(event Custom|forceUnequipBird
  (params (index :type Integer) (item :type Game%20Item%20Object%20Reference) (dstInventory :type Item%20Inventory%20Object%20Reference) (dstIndex :type Integer))
  ;[0.8878 1 0 0.5] Bird State Manipulation
  (Utilities|And+Branch (== item (Variables|RACO|birds|GetequippedBird)) (not (Utilities|Array|ContainsItem (RACO|birds|GetPermittedInventoriesforEquippedBirds) dstInventory))
    (:True
      (RACO|birds|DoUnequipBird))))

(event Custom|OpenDocumentGUI
  (params (paperObject :type Object%20Object%20Reference) (document :type STRUCT%20RACO%20Document%20Structure))
  ;[0.15 0.15 0.15 0.4] GUI: Document
  (bind _asbp_raco_i_paper_object (Utilities|Casting|CastToBP_RACO_I_PaperObject paperObject))
  (bind _modulename (Default|GetDocUIModuleName _asbp_raco_i_paper_object))
  (bind _returnvalue (Class|GUIModuleController|ActivateModule (Class|GUIModuleController|GetGUIModuleController) _modulename true false))
  (bind _asw_raco_document_gui (Utilities|Casting|CastToW_RACO_DocumentGUI _returnvalue))
  (Default|InitDocumentGUI _asw_raco_document_gui paperObject document))

(event Custom|reqSendMessage
  (params (senderEndpoint :type Actor%20Component%20Object%20Reference) (courier :type Game%20Item%20Ref%20Structure) (payload :type Array%20of%20Game%20Item%20Ref%20Structures) (recipientID :type String))
  ;[0.15 0.15 0.15 0.4] GUI: Mailbox and Coop
  (bind _item (CallFunction|ResolveGameItemRef courier))
  (bind _items (CallFunction|ResolveGameItemRefArray payload))
  (bind (_accepted _infomessage) (Class|BPRACOIMessagingEndpoint|TrySendMessage(Message) senderEndpoint (Utilities|GetConanCharacter) _item _items recipientID))
  (CallFunction|ClientExecutionResultCallback _accepted _infomessage))

(event Custom|TrackingLoop
  ;[0.05805 1 0.1022] Tracking
  (if (CallFunction|HasValidBirdID (Variables|RACO|birds|GetequippedBirdProfile))
    (Default|PerformTracking (Utilities|Array|Get(acopy) (stale Custom|toggleTrackingClient _outactors)) self)
    (else
      (CallFunction|ToggleTrackingClient))))

(event Custom|scanInventoryForDocs
  (params (inventory :type Item%20Inventory%20Object%20Reference))
  ;[1 0.03794 0.3524 0.3] Document client syncing
  ;;[0.15 0.15 0.15 0.5] Is this only needed for short and long item descriptions? (potentially weak reason)
  (bind _returnvalue (Class|ItemInventory|GetItemCount inventory))
  (Variables|Default|SettempCounter 0)
  (while (< (Variables|Default|GettempCounter) _returnvalue)
    (CallFunction|ReqUpdateItemDoc (Class|ItemInventory|GetItem inventory (Variables|Default|GettempCounter)))
    (Math|Integer|IncrementInt (Variables|Default|GettempCounter))))

(event Custom|clientExecutionResultCallback
  (params (success :type Boolean) (infoText :type String))
  ;[0.15 0.15 0.15 0.4] Callbacks
  (Default|CallExecutionResultCallback success infoText)
  (EventDispatchers|UnbindallEventsfromExecutionResultCallback))

(event Custom|OnSignalUpdateStats
  (params (updatedProfile :type STRUCT%20RACO%20Bird%20Profile%20Structure))
  ;[1 1 1] Bird UI Interaction
  (EventDispatchers|BindEventtoBirdProfileCallback (delegate Custom|OnBirdStatsUpdated))
  (CallFunction|ReqUpdateBirdStats (CallFunction|ConstructObjectRef 0) updatedProfile))

(event Custom|reqUpdateBirdStats
  (params (birdObject :type STRUCT%20RACO%20Agnostic%20Object%20Ref%20Structure) (deltaStats :type STRUCT%20RACO%20Bird%20Profile%20Structure))
  ;[0.8878 1 0 0.5] Bird State Manipulation
  (bind _object (CallFunction|ResolveObjectRef birdObject))
  (bind _birdprofile (Class|BPRACOIBird|GetBirdProfile(Message) _object))
  (bind (_success _updatedprofile) (CallFunction|UpdateBirdStats _birdprofile deltaStats))
  (if _success
    (Class|BPRACOIBird|SetBirdProfile(Message) _object _updatedprofile)
    (CallFunction|ClientBirdProfileCallback (CallFunction|ConstructObjectRef _object) _updatedprofile)))

(event Custom|reqGetBirdProfile
  (params (itemRef :type Game%20Item%20Ref%20Structure))
  ;[0.15 0.15 0.15 0.4] GUI: Mailbox and Coop
  (bind _item (CallFunction|ResolveGameItemRef itemRef))
  (bind _asbp_raco_i_bird (Utilities|Casting|CastToBP_RACO_I_Bird _item))
  (bind _birdprofile (Default|GetBirdProfile _asbp_raco_i_bird))
  (CallFunction|ClientBirdProfileCallback (CallFunction|ConstructObjectRef _item) _birdprofile))

(event Custom|clientBirdProfileCallback
  (params (birdObject :type STRUCT%20RACO%20Agnostic%20Object%20Ref%20Structure) (birdProfile :type STRUCT%20RACO%20Bird%20Profile%20Structure))
  ;[0.15 0.15 0.15 0.4] Callbacks
  (Default|CallBirdProfileCallback (CallFunction|ResolveObjectRef birdObject) birdProfile)
  (EventDispatchers|UnbindallEventsfromBirdProfileCallback))

(event Custom|OpenDocumentGUIFromClient
  (params (paperObject :type Object%20Object%20Reference))
  ;[0.15 0.15 0.15 0.4] GUI: Document
  (EventDispatchers|BindEventtoDocumentCallback (delegate Custom|OpenDocumentGUI))
  (CallFunction|ReqGetDocument (CallFunction|ConstructObjectRef paperObject) false true))

(event Custom|UpdateBirdDetectionConfig
  (params (birdPlaceable :type Object%20Object%20Reference) (config :type STRUCT%20RACO%20Bird%20Detection%20Config%20Structure))
  ;[1 1 1] Bird UI Interaction
  (Class|BPRACOIBird|SetDetectionConfig(Message) birdPlaceable config))

(event Custom|reqDocPickUp
  (params (placeable :type BP%20Master%20Placeables%20Object%20Reference))
  ;[1 0.125 0.125] Document Placeable handling
  (if (CallFunction|CanPickUpDocument (Utilities|GetConanCharacter) placeable)
    (bind _templateid (Class|BPRACOIPaperObject|GetPaperItemTemplateID(Message) placeable))
    (bind _returnvalue (Class|ItemInventory|AddItemTemplate (Utilities|GetCharacterInventory "Backpack") _templateid -1 "None" 1 false 1.0 -1.0))
    (bind _document (Class|BPRACOIPaperObject|GetDocument(Message) placeable))
    (Class|BPRACOIPaperObject|SetDocument(Message) (Class|ItemInventory|GetItem (Utilities|GetCharacterInventory "Backpack") _returnvalue) _document)
    (Actor|DestroyActor placeable)))

(event Custom|OnBirdStatsUpdated
  (params (birdObject :type Object%20Object%20Reference) (birdProfile :type STRUCT%20RACO%20Bird%20Profile%20Structure))
  ;[1 1 1] Bird UI Interaction
  (EventDispatchers|UnbindEventfromBirdProfileCallback (delegate Custom|OnBirdStatsUpdated))
  (Default|InitUI (Variables|Default|GetactiveBirdProfileUI) 0 birdProfile false))

(event Custom|clientOpenBirdProfile
  (params (birdObject :type Object%20Object%20Reference))
  ;[1 1 1] Bird UI Interaction
  (EventDispatchers|BindEventtoBirdProfileCallback (delegate Custom|OnBirdProfileReceived))
  (CallFunction|ReqGetBirdProfile000 (CallFunction|ConstructObjectRef birdObject)))

(event Custom|openBirdGUIFromClient
  (params (birdObject :type Object%20Object%20Reference))
  (EventDispatchers|BindEventtoBirdProfileCallback (delegate Custom|OnBirdProfileReceived))
  (CallFunction|ReqGetBirdProfile000 (CallFunction|ConstructObjectRef birdObject)))

(event Custom|reqGetDocument
  (params (paperObject :type STRUCT%20RACO%20Agnostic%20Object%20Ref%20Structure) (truncate :type Boolean) (callback :type Boolean))
  ;[0.15 0.15 0.15 0.4] GUI: Document
  (bind _object (CallFunction|ResolveObjectRef paperObject))
  (bind _asbp_raco_i_paper_object (Utilities|Casting|CastToBP_RACO_I_PaperObject _object))
  (bind _document (Default|GetDocument _asbp_raco_i_paper_object))
  (RACO|documents|SendDocUpdatetoClient _object _document truncate callback))

(event Custom|OnBirdProfileUIClosing
  (params (window :type Window%20Root%20Object%20Reference))
  ;[1 1 1] Bird UI Interaction
  (Variables|Default|SetactiveBirdProfileUI 0)
  (CallFunction|DisposeBirdPreview))

(event Custom|reqStartPlacement
  (params (birdItem :type Game%20Item%20Ref%20Structure))
  (bind _conancharacter (Utilities|GetConanCharacter))
  ;[0.8878 1 0 0.5] Bird State Manipulation
  (bind _asbp_base_bird_item (Utilities|Casting|CastToBP_BaseBirdItem (CallFunction|ResolveGameItemRef birdItem)))
  (bind _birdprofile (Class|BPRACOIBird|GetBirdProfile(Message) _asbp_base_bird_item))
  (Variables|RACO|birds|SetbirdProfileBeingPlaced _birdprofile)
  (Default|TriggerStartPlacement _asbp_base_bird_item _conancharacter _conancharacter))

(event Custom|notifyItemBeingPlaced
  (params (itemRef :type STRUCT%20RACO%20Agnostic%20Object%20Ref%20Structure))
  ;[1 0.125 0.125] Document Placeable handling
  (bind _object (CallFunction|ResolveObjectRef itemRef))
  (bind _templateid (Class|BPRACOIPaperObject|GetPaperItemTemplateID(Message) _object))
  (Variables|RACO|documents|SetdocTemplateID _templateid)
  (bind _document (Class|BPRACOIPaperObject|GetDocument(Message) _object))
  (Variables|RACO|documents|SetdocBeingPlaced _document))

(event Custom|clientOpenBirdProfile2
  (params (profile :type STRUCT%20RACO%20Bird%20Profile%20Structure))
  ;[1 1 1] Bird UI Interaction
  (CallFunction|PrepareBirdPreview profile)
  (bind _windowroot (|GUIModuleControllerActivate (Class|GUIModuleController|GetGUIModuleController) "RACO_ViewBirdProfile" true false)
    (:OnActivate
      (bind _output_get (Variables|Default|SetactiveBirdProfileUI (.AsW%20RACO%20Bird%20Profile%20View (Utilities|Casting|CastToW_RACO_BirdProfileView _windowroot))))
      (Default|InitUI _output_get 0 profile true)
      (EventDispatchers|BindEventtoSignalClosing _windowroot (delegate Custom|OnBirdProfileUIClosing)))))

(event Custom|OnSignalPlaceBird
  (bind _conancharacter (Utilities|GetConanCharacter))
  ;[1 1 1] Bird UI Interaction
  (CallFunction|ReqStartPlacement (CallFunction|ConstructGameItemRef 0))
  (Default|TriggerStartPlacement (.AsBP%20Base%20Bird%20Item (Utilities|Casting|CastToBP_BaseBirdItem 0)) _conancharacter _conancharacter))

(event Custom|clientEquippedBirdCallback
  ;[0.15 0.15 0.15 0.4] Callbacks
)

(event Custom|notifyItemPlacementDone
  (bind _returnvalue (Components|GetOwner))
  (bind _returnvalue_2 (Actor|GetComponentbyClass _returnvalue "/Game/Systems/Building/BP_BuildSystem_v2.BP_BuildSystem_v2_C"))
  ;[1 0.125 0.125] Document Placeable handling
  (if (Variables|/Script/ConanSandbox.BuildSystemComponent|GetIsBuilding _returnvalue_2)
    (Class|BuildSystemComponent|StopBuilding _returnvalue_2)))

(event Custom|reqToggleEquippedBird
  (params (birdObject :type STRUCT%20RACO%20Agnostic%20Object%20Ref%20Structure))
  ;[0.8878 1 0 0.5] Bird State Manipulation
  (bind _object (CallFunction|ResolveObjectRef birdObject))
  (if (CallFunction|IsBird _object)
    (if (== _object (Variables|RACO|birds|GetequippedBird))
      (RACO|birds|DoUnequipBird)
      (else
        (bind _asgame_item (Utilities|Casting|CastToGameItem _object))
        (if (Utilities|Array|ContainsItem (RACO|birds|GetPermittedInventoriesforEquippedBirds) (Class|GameItem|GetOwnerInventory _asgame_item))
          (RACO|birds|DoEquipBird _asgame_item))))))

(event Custom|clientOpenBirdDetectionConfig
  (params (birdPlaceable :type Object%20Object%20Reference))
  ;[1 1 1] Bird UI Interaction
  (bind _returnvalue (Class|BPRACOIBird|GetDetectionConfig(Message) birdPlaceable))
  (bind _birdprofile (Class|BPRACOIBird|GetBirdProfile(Message) birdPlaceable))
  (bind _windowroot (|GUIModuleControllerActivate (Class|GUIModuleController|GetGUIModuleController) "RACO_ViewBirdDetectionConfig" true false)
    (:OnActivate
      (Default|InitUI (.AsW%20Bird%20Detection%20Config%20View (Utilities|Casting|CastToW_BirdDetectionConfig_View _windowroot)) _birdprofile _returnvalue)
      (EventDispatchers|BindEventtoSignalUpdateConfig (.AsW%20Bird%20Detection%20Config%20View (Utilities|Casting|CastToW_BirdDetectionConfig_View _windowroot)) (delegate Custom|OnSignalUpdateConfig)))))

(event Custom|clientUpdateItemDoc
  (params (paperObjectRef :type STRUCT%20RACO%20Agnostic%20Object%20Ref%20Structure) (document :type STRUCT%20RACO%20Document%20Structure) (triggerCallback :type Boolean))
  ;[0.15 0.15 0.15 0.4] GUI: Document
  (bind _object (CallFunction|ResolveObjectRef paperObjectRef))
  (Class|BPRACOIPaperObject|SetDocument(Message) _object document)
  (if triggerCallback
    (CallFunction|ClientDocumentCallback _object document)))

(event Custom|LoopBirdRandomAnimation
  (bind _equippedbirdprofile (Variables|RACO|birds|GetequippedBirdProfile))
  (bind _birdtypeid (Utilities|Struct|BreakSTRUCT_RACO_BirdProfile _equippedbirdprofile))
  ;[0.8878 1 0 0.5] Bird State Manipulation
  (if (Math|Boolean|NORBoolean (Networking|IsDedicatedServer) (Utilities|Array|IsEmpty (Utilities|String|ToString(Name) _birdtypeid)))
    (bind (_success _animlength) (CallFunction|PlayRandomBirdAnimation (Variables|Default|GetequippedBirdMesh) _birdtypeid true))
    (if _success
      (Utilities|FlowControl|Delay (+ _animlength (Math|Random|RandomFloatinRange 2.0 5.0)))
      (CallFunction|LoopBirdRandomAnimation))))

(event Custom|toggleTrackingClient
  ;[0.05805 1 0.1022] Tracking
  (if (Default|GetIsTrackingAllowed (CallFunction|GetServerSettingsRACO))
    (bind _output_get (Variables|Default|SetisTrackingActive (not (Class|GUIModuleController|IsModuleActive (Class|GUIModuleController|GetGUIModuleController) "RACO_Tracking_HUD"))))
    (bind _returnvalue (Class|GUIModuleController|ActivateModule (Class|GUIModuleController|GetGUIModuleController) "RACO_Tracking_HUD" _output_get false))
    (if (Variables|Default|GetisTrackingActive)
      (bind _outactors (Actor|GetAllActorsOfClass "/Game/Mods/RavencrestCouriers/System/BP_RACO_A_TrackingSystem.BP_RACO_A_TrackingSystem_C"))
      (Default|InitHUD (.AsW%20Tracking%20HUD (Utilities|Casting|CastToW_Tracking_HUD _returnvalue)) (Utilities|Array|Get(acopy) _outactors))
      (bind _returnvalue_2 (Utilities|Time|SetTimerbyEvent (delegate Custom|TrackingLoop) 5.0 true))
      (Variables|Default|SettrackingTimer _returnvalue_2)
      (else
        (Utilities|Time|ClearandInvalidateTimerbyHandle (Variables|Default|GettrackingTimer))))
    (else
      (bind _returnvalue_3 (Class|MessageBoxWidget|CreateMessageBox (Components|GetOwner) "OK" "Tracking Disabled" "Bird Tracking has been disabled on this server."))
      (Class|MessageBoxWidget|ShowMessageBox _returnvalue_3 0 1001))))

(event Custom|OnBirdToggleTracking
  ;[1 1 1] Bird UI Interaction
  (CallFunction|ToggleTrackingClient))

(event Custom|OpenDocumentGUIfromServer
  (params (paperObject :type Object%20Object%20Reference) (document :type STRUCT%20RACO%20Document%20Structure))
  ;[0.15 0.15 0.15 0.4] GUI: Document
  (CallFunction|OpenDocumentGUI paperObject (RACO|documents|RedactDocument document false)))

(event Custom|reqGetBirdProfile000
  (params (birdObject :type STRUCT%20RACO%20Agnostic%20Object%20Ref%20Structure))
  (bind _object (CallFunction|ResolveObjectRef birdObject))
  (bind _birdprofile (Class|BPRACOIBird|GetBirdProfile(Message) _object))
  (CallFunction|ClientBirdProfileCallback (CallFunction|ConstructObjectRef _object) _birdprofile))

(event Custom|OnBirdProfileReceived
  (params (birdObject :type Object%20Object%20Reference) (birdProfile :type STRUCT%20RACO%20Bird%20Profile%20Structure))
  ;[1 1 1] Bird UI Interaction
  (CallFunction|PrepareBirdPreview birdProfile)
  (bind _windowroot (|GUIModuleControllerActivate (Class|GUIModuleController|GetGUIModuleController) "RACO_ViewBirdProfile" true false)
    (:OnActivate
      (bind _output_get (Variables|Default|SetactiveBirdProfileUI (.AsW%20RACO%20Bird%20Profile%20View (Utilities|Casting|CastToW_RACO_BirdProfileView _windowroot))))
      (Default|InitUI _output_get 0 birdProfile false)
      (EventDispatchers|BindEventtoSignalPlaceBird (Variables|Default|GetactiveBirdProfileUI) (delegate Custom|OnSignalPlaceBird))
      (EventDispatchers|BindEventtoSignalUpdateStats (Variables|Default|GetactiveBirdProfileUI) (delegate Custom|OnSignalUpdateStats))
      (EventDispatchers|BindEventtoSignalClosing (Variables|Default|GetactiveBirdProfileUI) (delegate Custom|OnBirdProfileUIClosing))
      (EventDispatchers|BindEventtoSignalToggleTracking (Variables|Default|GetactiveBirdProfileUI) (delegate Custom|OnBirdToggleTracking)))))

(event Custom|reqChangeBirdName
  (params (birdObject :type STRUCT%20RACO%20Agnostic%20Object%20Ref%20Structure) (newName :type String))
  ;[0.8878 1 0 0.5] Bird State Manipulation
  (bind _object (CallFunction|ResolveObjectRef birdObject))
  (bind _birdprofile (Class|BPRACOIBird|GetBirdProfile(Message) _object))
  (bind _structout (Utilities|Struct|SetmembersinSTRUCT_RACO_BirdProfile _birdprofile newName))
  (Class|BPRACOIBird|SetBirdProfile(Message) _object _structout)
  (CallFunction|ClientBirdProfileCallback (CallFunction|ConstructObjectRef _object) _structout))

(event Custom|reqToggleCanReceive
  (params (endpoint :type Actor%20Component%20Object%20Reference) (canReceive :type Boolean))
  ;[0.15 0.15 0.15 0.4] GUI: Mailbox and Coop
  (Class|BPRACOIMessagingEndpoint|SetCanReceive(Message) endpoint canReceive))

(event Custom|clientDocumentCallback
  (params (paperObject :type Object%20Object%20Reference) (document :type STRUCT%20RACO%20Document%20Structure))
  ;[0.15 0.15 0.15 0.4] Callbacks
  (Default|CallDocumentCallback paperObject document)
  (EventDispatchers|UnbindallEventsfromDocumentCallback))

(event Custom|reqUpdateItemDoc
  (params (item :type Game%20Item%20Object%20Reference))
  ;[1 0.03794 0.3524 0.3] Document client syncing
  ;;[0.15 0.15 0.15 0.5] Is this only needed for short and long item descriptions? (potentially weak reason)
  (bind _asbp_raco_i_paper_object (Utilities|Casting|CastToBP_RACO_I_PaperObject item))
  (bind _document (Default|GetDocument _asbp_raco_i_paper_object))
  (RACO|documents|SendDocUpdatetoClient item _document false false))

(event Custom|reqDepositItems
  (params (endpoint :type Actor%20Component%20Object%20Reference) (items :type Array%20of%20Game%20Item%20Ref%20Structures))
  ;[0.15 0.15 0.15 0.4] GUI: Mailbox and Coop
  (bind (_success _infomessage) (Class|BPRACOIMessagingEndpoint|TryDepositItems(Message) endpoint (Utilities|GetConanCharacter) (CallFunction|ResolveGameItemRefArray items)))
  (CallFunction|ClientExecutionResultCallback _success _infomessage))

(event Custom|reqSaveDocument
  (params (paperObject :type STRUCT%20RACO%20Agnostic%20Object%20Ref%20Structure) (document :type STRUCT%20RACO%20Document%20Structure))
  ;[0.15 0.15 0.15 0.4] GUI: Document
  (bind _object (CallFunction|ResolveObjectRef paperObject))
  (bind (_success _infomessage) (Class|BPRACOIPaperObject|TryApplyEdits(Message) _object (Utilities|GetPlayerController) document))
  (Class|ConanCharacter|ClientHUDShowNotification (Utilities|GetConanCharacter) (Utilities|Text|ToText(String) _infomessage) _success true)
  (if _success
    (RACO|documents|SendDocUpdatetoClient _object document false false)))

(event Custom|InitInventoryDocSync
  (bind _inventory (Utilities|GetCharacterInventory "ShortcutBar"))
  (bind _inventory_2 (Utilities|GetCharacterInventory "Backpack"))
  ;[1 0.03794 0.3524 0.3] Document client syncing
  ;;[0.15 0.15 0.15 0.5] Is this only needed for short and long item descriptions? (potentially weak reason)
  (EventDispatchers|BindEventtoSignalItemAdded _inventory_2 (delegate Custom|OnItemAdded))
  (CallFunction|ScanInventoryforDocs _inventory_2)
  (EventDispatchers|BindEventtoSignalItemAdded _inventory (delegate Custom|OnItemAdded))
  (CallFunction|ScanInventoryforDocs _inventory))

(event Custom|reqPickupBird
  (params (birdPlaceable :type Actor%20Object%20Reference))
  (bind _inventory (Utilities|GetCharacterInventory "Backpack"))
  ;[0.8878 1 0 0.5] Bird State Manipulation
  (bind _templateid (Class|BPRACOIBird|GetBirdTemplateID(Message) birdPlaceable))
  (bind _returnvalue (Class|ItemInventory|AddItemTemplate _inventory _templateid -1 "None" 1 false 1.0 -1.0))
  (bind _birdprofile (Class|BPRACOIBird|GetBirdProfile(Message) birdPlaceable))
  (Class|BPRACOIBird|SetBirdProfile(Message) (Class|ItemInventory|GetItem _inventory _returnvalue) _birdprofile)
  (Utilities|FlowControl|Sequence
    (:then_0
      (bind _returnvalue_2 (Actor|GetComponentsByClass birdPlaceable "/Script/UE4Dreamworld.PersistenceComponent"))
      (bind _array_element (Utilities|ForEachLoopFast _returnvalue_2)
        (:LoopBody
          (Class|PersistenceComponent|Delete _array_element))))
    (:then_1
      (Actor|DestroyActor birdPlaceable))))

(event Custom|reqGetMessagingDestinations
  (params (endpoint :type Actor%20Component%20Object%20Reference))
  ;[0.15 0.15 0.15 0.4] GUI: Mailbox and Coop
  (bind _destinations (Class|BPRACOIMessagingSystem|GetListOfDestinations(Message) (CallFunction|GetModControllerRACO) endpoint))
  (CallFunction|ClientDestinationsCallback _destinations))

(event Custom|reqNestBird
  (params (nest :type Actor%20Object%20Reference) (bird :type Game%20Item%20Ref%20Structure))
  ;[0.15 0.15 0.15 0.4] GUI: Mailbox and Coop
  (bind (_success _infomessage) (Class|BPRACOINest|TryNestBird(Message) nest (CallFunction|ResolveGameItemRef bird)))
  (CallFunction|ClientExecutionResultCallback _success _infomessage))

(event Custom|clientDestinationsCallback
  (params (destinations :type Array%20of%20Strings))
  ;[0.15 0.15 0.15 0.4] Callbacks
  (Default|CallDestinationsCallback destinations)
  (EventDispatchers|UnbindallEventsfromDestinationsCallback))

(event Custom|OnSignalUpdateConfig
  (params (updatedConfig :type STRUCT%20RACO%20Bird%20Detection%20Config%20Structure))
  ;[1 1 1] Bird UI Interaction
  (CallFunction|UpdateBirdDetectionConfig (stale Custom|clientOpenBirdDetectionConfig birdPlaceable) updatedConfig))

(event Custom|reqCopyDocumentItem
  (params (copy :type STRUCT%20RACO%20Agnostic%20Object%20Ref%20Structure) (original :type STRUCT%20RACO%20Agnostic%20Object%20Ref%20Structure))
  ;[0.15 0.15 0.15 0.4] GUI: Document
  (bind _object (CallFunction|ResolveObjectRef copy))
  (bind (_success _infomessage) (Class|BPRACOIPaperObject|TryMakeCopy(Message) _object (CallFunction|ResolveObjectRef original) (Utilities|GetPlayerController)))
  (Class|ConanCharacter|ClientHUDShowNotification (Utilities|GetConanCharacter) (Utilities|Text|ToText(String) _infomessage) _success true)
  (if _success
    (bind _document (Class|BPRACOIPaperObject|GetDocument(Message) _object))
    (RACO|documents|SendDocUpdatetoClient _object _document true false)))

(event Custom|reqBreakSeal
  (params (paperObjectRef :type STRUCT%20RACO%20Agnostic%20Object%20Ref%20Structure))
  ;[0.15 0.15 0.15 0.4] GUI: Document
  (bind _object (CallFunction|ResolveObjectRef paperObjectRef))
  (bind (_success _infomessage) (Class|BPRACOIPaperObject|TryBreakSeal(Message) _object))
  (Class|ConanCharacter|ClientHUDShowNotification (Utilities|GetConanCharacter) (Utilities|Text|ToText(String) _infomessage) _success true)
  (if _success
    (bind _document (Class|BPRACOIPaperObject|GetDocument(Message) _object))
    (RACO|documents|SendDocUpdatetoClient _object _document false true)))

(event Custom|OnItemAdded
  (params (index :type Integer) (item :type Game%20Item%20Object%20Reference) (srcInventory :type Item%20Inventory%20Object%20Reference) (srcIndex :type Integer))
  ;[1 0.03794 0.3524 0.3] Document client syncing
  ;;[0.15 0.15 0.15 0.5] Is this only needed for short and long item descriptions? (potentially weak reason)
  (CallFunction|ReqUpdateItemDoc item))

(event EventEndPlay
  (params (EndPlayReason :type EEndPlayReason%20Enum :default "Destroyed"))
  (if (Networking|IsServer)
    (Variables|RACO|birds|GetequippedBird
      (:then
        (RACO|birds|DoUnequipBird))
      (:else))))

(event EventBeginPlay
  (if (Networking|IsServer)
    _))

(fn PrepareBirdPreview
  (params (birdProfile :type STRUCT%20RACO%20Bird%20Profile%20Structure))
  (Utilities|FlowControl|Sequence
    (:then_0
      (Utilities|IsValid (Variables|RACO|birds|GetbirdPreviewRoom)
        (:Is%20Not%20Valid
          (bind _returnvalue (Game|SpawnActorfromClass "/Game/Mods/RavencrestCouriers/UI/bird_preview/BP_RACO_PreviewRoom.BP_RACO_PreviewRoom_C" (Math|Conversions|ToTransform(Vector) "0, 0,-15000.000000") "Undefined" "OverrideRootScale" (Components|GetOwner) 0))
          (Variables|RACO|birds|SetbirdPreviewRoom _returnvalue))))
    (:then_1
      (Default|RefreshBirdMesh (Variables|RACO|birds|GetbirdPreviewRoom) (Utilities|Struct|BreakSTRUCT_RACO_BirdProfile birdProfile)))))

(fn DisposeBirdPreview
  (Utilities|IsValid (Variables|RACO|birds|GetbirdPreviewRoom)
    (:Is%20Valid
      (Actor|DestroyActor (Variables|RACO|birds|GetbirdPreviewRoom))
      (Variables|RACO|birds|SetbirdPreviewRoom 0))))

(fn OnRepEquippedBirdProfile
  (bind _equippedbirdprofile (Variables|RACO|birds|GetequippedBirdProfile))
  (bind _birdtypeid (Utilities|Struct|BreakSTRUCT_RACO_BirdProfile _equippedbirdprofile))
  (bind _birdtype (CallFunction|GetBirdTypebyID _birdtypeid))
  (bind (_skeletalmesh _transform) (Utilities|Struct|BreakSTRUCT_RACO_BirdType _birdtype))
  (Utilities|FlowControl|Sequence
    (:then_0
      (bind _output_get (LocalVariables|Setcharacter (Utilities|GetConanCharacter)))
      (Utilities|IsValid _output_get
        (:Is%20Valid
          (LocalVariables|SetcharacterGender (Class|ConanCharacter|GetIntStat _output_get "Gender" "Full")))))
    (:then_1
      (Utilities|IsValid (Variables|Default|GetequippedBirdMesh)
        (:Is%20Not%20Valid
          (bind _returnvalue (Class|CharacterFunctionLibrary|AddSkeletalMeshComponent (LocalVariables|Getcharacter) true (Utilities|Select :Index (- (LocalVariables|GetcharacterGender) 1) :Option%200 (LocalVariables|GetmaleTransform) :Option%201 (LocalVariables|GetfemaleTransform)) "/Script/Engine.SkeletalMeshComponent"))
          (bind _output_get_2 (Variables|Default|SetequippedBirdMesh _returnvalue))
          (Transformation|AttachComponentToComponent _output_get_2 (Variables|/Script/Engine.Character|GetMesh (LocalVariables|Getcharacter)) "b_R_clavicle" "KeepRelative" "KeepRelative" "KeepRelative" true))))
    (:then_2
      (if (CallFunction|HasValidBirdID _equippedbirdprofile)
        (Transformation|SetRelativeTransform (Variables|Default|GetequippedBirdMesh) (Math|Transform|ComposeTransforms (Utilities|Select :Index (- (LocalVariables|GetcharacterGender) 1) :Option%200 (LocalVariables|GetmaleTransform) :Option%201 (LocalVariables|GetfemaleTransform)) _transform) false false)
        (Components|SkinnedMesh|SetSkinnedAssetandUpdate (Variables|Default|GetequippedBirdMesh) _skeletalmesh true)
        (CallFunction|LoopBirdRandomAnimation)
        (else
          (Components|SkinnedMesh|SetSkinnedAssetandUpdate (Variables|Default|GetequippedBirdMesh) 0 true))))
    (:then_3
      (Utilities|And+Branch (not (Networking|IsDedicatedServer)) (Pawn|IsLocallyControlled (Utilities|GetConanCharacter))
        (:True
          (Default|CallEquippedBirdChangedonClient))))))

(fn IsBirdEquipped
  (params (profileGUID :type Guid%20Structure))
  (return (== profileGUID (Utilities|Struct|BreakSTRUCT_RACO_BirdProfile (Variables|RACO|birds|GetequippedBirdProfile)))))

(fn RedactDocument
  (params (document :type STRUCT%20RACO%20Document%20Structure) (Truncate :type Boolean))
  (bind _text (Utilities|Struct|BreakSTRUCT_RACO_Document document))
  (Utilities|FlowControl|Sequence
    (:then_0
      (if (Utilities|Struct|BreakSTRUCT_RACO_Document document)
        (bind _output_get (LocalVariables|SetlocalDocument document))
        (bind _structout (Utilities|Struct|SetmembersinSTRUCT_RACO_Document _output_get "" "" "" (Utilities|Array|MakeArray)))
        (return _structout)))
    (:then_1
      (if Truncate
        (if (not (Utilities|Array|IsEmpty _text))
          (bind _output_get_2 (LocalVariables|SetlocalDocument document))
          (bind _structout_2 (Utilities|Struct|SetmembersinSTRUCT_RACO_Document _output_get_2 (Utilities|Array|MakeArray (Utilities|String|Left (Utilities|Array|Get(acopy) _text) (+ (CallFunction|GetDescriptionLength false) 10)))))
          (return _structout_2))))
    (:then_2
      (return document))))

(fn SendDocUpdatetoClient
  (params (paperObject :type Object%20Object%20Reference) (document :type STRUCT%20RACO%20Document%20Structure) (truncate :type Boolean) (callback :type Boolean))
  (CallFunction|ClientUpdateItemDoc (CallFunction|ConstructObjectRef paperObject) (RACO|documents|RedactDocument document truncate) callback))

(fn DoEquipBird
  (params (bird :type Object%20Object%20Reference))
  (bind _output_get (Variables|RACO|birds|SetequippedBird bird))
  (bind _birdprofile (Class|BPRACOIBird|GetBirdProfile(Message) _output_get))
  (Variables|RACO|birds|SetequippedBirdProfile _birdprofile)
  (Variables|RACO|birds|SetequippedBirdStartTime (Math|DateTime|UTCNow))
  (EventDispatchers|BindEventtoSignalItemRemoved (RACO|birds|GetPermittedInventoriesforEquippedBirds) (EventDispatchers|CreateEvent :!event Custom|forceUnequipBird)))

(fn DoUnequipBird
  (Utilities|FlowControl|Sequence
    (:then_0
      (if (not (== (Variables|RACO|birds|GetequippedBirdStartTime) (CallFunction|MakeInvalidDatetime)))
        (Default|GiveBirdPassiveXP (CallFunction|GetExperienceSystemRACO) (Variables|RACO|birds|GetequippedBird) (Math|Timespan|GetTotalHours (- (Math|DateTime|UTCNow) (Variables|RACO|birds|GetequippedBirdStartTime))))))
    (:then_1
      (Variables|RACO|birds|SetequippedBird 0)
      (Variables|RACO|birds|SetequippedBirdProfile "")
      (Variables|RACO|birds|SetequippedBirdStartTime (CallFunction|MakeInvalidDatetime))
      (EventDispatchers|UnbindEventfromSignalItemRemoved (RACO|birds|GetPermittedInventoriesforEquippedBirds) (EventDispatchers|CreateEvent :!event Custom|forceUnequipBird)))))

(fn GetPermittedInventoriesforEquippedBirds
  (return (Utilities|Array|MakeArray (Utilities|GetCharacterInventory "ShortcutBar"))))