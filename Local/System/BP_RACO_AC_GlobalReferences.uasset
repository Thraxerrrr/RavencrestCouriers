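; BP_RACO_AC_GlobalReferences is a component that provides shared lookups for the RACO mod's controller and its systems.
; GetModController lazily finds the first actor implementing the BP_RACO_I_MessagingSystem interface and caches it, searching again only when the cached reference is invalid.
; The ServerSettings and ExperienceSystem getters fetch their components by class from that controller.
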(fn GetModController
  (Variables|Default|GetRACO_ModController
    (:then
      _)
    (:else
      (bind _outactors (Actor|GetAllActorswithInterface "/Game/Mods/RavencrestCouriers/System/BP_RACO_I_MessagingSystem.BP_RACO_I_MessagingSystem_C"))
      (Variables|Default|SetRACO_ModController (Utilities|Array|Get(acopy) _outactors))))
  (return (Variables|Default|GetRACO_ModController)))

(fn GetServerSettingsAC
  (return (Actor|GetComponentbyClass (CallFunction|GetModController) "/Game/Mods/RavencrestCouriers/System/BP_RACO_AC_ServerSettings.BP_RACO_AC_ServerSettings_C")))

(fn GetExperienceSystemAC
  (return (Actor|GetComponentbyClass (CallFunction|GetModController) "/Game/Mods/RavencrestCouriers/System/BP_RACO_AC_ExperienceSystem.BP_RACO_AC_ExperienceSystem_C")))