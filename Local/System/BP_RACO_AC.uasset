(event Custom|forceUnequipBird
  (params (index :type Integer) (item :type Game%20Item%20Object%20Reference) (dstInventory :type Item%20Inventory%20Object%20Reference) (dstIndex :type Integer))
  ;[0.8878 1 0 0.5] Bird State Manipulation
  (Utilities|And+Branch (== item (Variables|Default|GetequippedBird)) (!= dstInventory (Utilities|GetCharacterInventory "ShortcutBar"))
    (:True
      (Variables|Default|SetequippedBird 0)
      (Variables|Default|SetequippedBirdProfile "")
      (EventDispatchers|UnbindEventfromSignalItemRemoved (Utilities|GetCharacterInventory "ShortcutBar") (delegate Custom|forceUnequipBird)))))

(event Custom|OpenDocumentGUI
  (params (paperObject :type Object%20Object%20Reference) (document :type STRUCT%20RACO%20Document%20Structure))
  ;[0.15 0.15 0.15 0.4] GUI: Document
  (bind _asbp_raco_i_document (Utilities|Casting|CastToBP_RACO_I_Document paperObject))
  (bind _modulename (Default|GetDocUIModuleName _asbp_raco_i_document))
  (bind _returnvalue (Class|GUIModuleController|ActivateModule (Class|GUIModuleController|GetGUIModuleController) _modulename true false))
  (bind _asw_raco_document_gui (Utilities|Casting|CastToW_RACO_DocumentGUI _returnvalue))
  (Default|InitDocument _asw_raco_document_gui paperObject document))

(event Custom|reqSendMessage
  (params (senderEndpoint :type Actor%20Component%20Object%20Reference) (carrier :type Game%20Item%20Ref%20Structure) (payload :type Array%20of%20Game%20Item%20Ref%20Structures) (recipientID :type String))
  ;[0.15 0.15 0.15 0.4] GUI: Mailbox and Coop
  (bind _item (CallFunction|ResolveGameItemRef carrier))
  (bind (_accepted _errorinfo) (Class|BPRACOIMessagingEndpoint|TrySendMessage(Message) senderEndpoint _item (CallFunction|ResolveGameItemRefArray payload) recipientID))
  (CallFunction|ClientExecutionResultCallback _accepted _errorinfo))

(event Custom|TrackingLoop
  ;[0.05805 1 0.1022] Tracking
  (if (CallFunction|IsValidBirdProfile (Variables|Default|GetequippedBirdProfile))
    (Default|PerformTracking (Utilities|Array|Get(acopy) (stale Custom|toggleTrackingClient _outactors)) self)
    (else
      (CallFunction|ToggleTrackingClient))))

(event Custom|scanInventoryForDocs
  (params (inventory :type Item%20Inventory%20Object%20Reference))
  ;[1 0.03794 0.3524 0.3] Document client syncing
  ;;[0.15 0.15 0.15 0.5] Is this only needed for short and long item descriptions? (potentially weak reason)
  (Variables|Default|SettempCounter 0)
  (while (< (Variables|Default|GettempCounter) (Class|ItemInventory|GetItemCount inventory))
    (CallFunction|ReqUpdateItemDoc (Class|ItemInventory|GetItem inventory (Variables|Default|GettempCounter)))
    (Math|Integer|IncrementInt (Variables|Default|GettempCounter))))

(event Custom|clientExecutionResultCallback
  (params (success :type Boolean) (infoText :type String))
  ;[0.15 0.15 0.15 0.4] Callbacks
  (Default|CallExecutionResultCallback success infoText)
  (EventDispatchers|UnbindallEventsfromExecutionResultCallback))

(event Custom|OnSignalUpdateStats
  (params (updatedProfile :type STRUCT%20RACO%20Bird%20Profile%20Structure))
  ;[1 1 1] Bird UI Interaction
  (EventDispatchers|BindEventtoBirdProfileCallback (delegate Custom|OnBirdStatsUpdated))
  (CallFunction|ReqUpdateBirdStats (CallFunction|ConstructGameItemRef (stale Custom|OnBirdProfileReceived itemRef)) updatedProfile))

(event Custom|reqUpdateBirdStats
  (params (itemRef :type Game%20Item%20Ref%20Structure) (updatedStats :type STRUCT%20RACO%20Bird%20Profile%20Structure))
  (bind (_travelspeedpoints _carryweightpoints _detectionrangepoints _unspentpoints) (Utilities|Struct|BreakSTRUCT_RACO_BirdProfile updatedStats))
  ;[0.8878 1 0 0.5] Bird State Manipulation
  (bind _item (CallFunction|ResolveGameItemRef itemRef))
  (bind _asbp_base_bird_item (Utilities|Casting|CastToBP_BaseBirdItem _item))
  (bind _structout (Utilities|Struct|SetmembersinSTRUCT_RACO_BirdProfile (Variables|/Game/Mods/RavencrestCouriers/Items/BP_BaseBirdItem.BP_BaseBirdItem_C|GetbirdProfile _asbp_base_bird_item) _travelspeedpoints _carryweightpoints _detectionrangepoints _unspentpoints))
  (bind _output_get (Variables|/Game/Mods/RavencrestCouriers/Items/BP_BaseBirdItem.BP_BaseBirdItem_C|SetbirdProfile _asbp_base_bird_item _structout))
  (CallFunction|ClientBirdProfileCallback itemRef _output_get))

(event Custom|reqGetBirdProfile
  (params (itemRef :type Game%20Item%20Ref%20Structure))
  ;[0.15 0.15 0.15 0.4] GUI: Mailbox and Coop
  (bind _item (CallFunction|ResolveGameItemRef itemRef))
  (bind _asbp_base_bird_item (Utilities|Casting|CastToBP_BaseBirdItem _item))
  (CallFunction|ClientBirdProfileCallback (CallFunction|ConstructGameItemRef _asbp_base_bird_item) (Variables|/Game/Mods/RavencrestCouriers/Items/BP_BaseBirdItem.BP_BaseBirdItem_C|GetbirdProfile _asbp_base_bird_item)))

(event Custom|clientBirdProfileCallback
  (params (itemRef :type Game%20Item%20Ref%20Structure) (birdProfile :type STRUCT%20RACO%20Bird%20Profile%20Structure))
  ;[0.15 0.15 0.15 0.4] Callbacks
  (bind _item (CallFunction|ResolveGameItemRef itemRef))
  (Default|CallBirdProfileCallback _item birdProfile)
  (EventDispatchers|UnbindallEventsfromBirdProfileCallback))

(event Custom|OpenDocumentGUIFromItem
  (params (item :type Game%20Item%20Ref%20Structure))
  ;[0.15 0.15 0.15 0.4] GUI: Document
  (EventDispatchers|BindEventtoDocumentCallback (delegate Custom|OpenDocumentGUI))
  (CallFunction|ReqGetDocumentfromItem item))

(event Custom|UpdateBirdDetectionConfig
  (params (config :type STRUCT%20RACO%20Bird%20Detection%20Config%20Structure) (birdPlaceable :type BP%20Base%20Bird%20Placeable%20Object%20Reference))
  ;[1 1 1] Bird UI Interaction
  (Default|UpdateDetectionConfig birdPlaceable config))

(event Custom|reqDocPickUp
  (params (placeable :type BP%20Base%20Document%20Placeable%20Object%20Reference))
  ;[1 0.125 0.125] Document Placeable handling
  (bind _templateid (Class|BPRACOIDocument|GetPaperItemTemplateID(Message) placeable))
  (bind _returnvalue (Class|ItemInventory|AddItemTemplate (Utilities|GetCharacterInventory "Backpack") _templateid -1 "None" 1 false 1.0 -1.0))
  (bind _document (Class|BPRACOIDocument|GetDocument(Message) placeable))
  (Class|BPRACOIDocument|SetDocument(Message) (Class|ItemInventory|GetItem (Utilities|GetCharacterInventory "Backpack") _returnvalue) _document)
  (Actor|DestroyActor placeable))

(event Custom|OnBirdStatsUpdated
  (params (itemRef :type Game%20Item%20Object%20Reference) (birdProfile :type STRUCT%20RACO%20Bird%20Profile%20Structure))
  ;[1 1 1] Bird UI Interaction
  (EventDispatchers|UnbindEventfromBirdProfileCallback (delegate Custom|OnBirdStatsUpdated))
  (Default|InitUI (Variables|Default|GetactiveBirdProfileUI) birdProfile false))

(event Custom|clientOpenBirdProfile
  (params (birdItem :type BP%20Base%20Bird%20Item%20Object%20Reference))
  ;[1 1 1] Bird UI Interaction
  (EventDispatchers|BindEventtoBirdProfileCallback (delegate Custom|OnBirdProfileReceived))
  (CallFunction|ReqGetBirdProfile000 (CallFunction|ConstructGameItemRef birdItem)))

(event Custom|reqGetDocumentFromItem
  (params (itemRef :type Game%20Item%20Ref%20Structure))
  ;[0.15 0.15 0.15 0.4] GUI: Document
  (bind _item (CallFunction|ResolveGameItemRef itemRef))
  (bind _asbp_raco_i_document (Utilities|Casting|CastToBP_RACO_I_Document _item))
  (bind _document (Default|GetDocument _asbp_raco_i_document))
  (CallFunction|SendDocUpdatetoClient _item _document true))

(event Custom|OnBirdProfileUIClosing
  (params (window :type Window%20Root%20Object%20Reference))
  ;[1 1 1] Bird UI Interaction
  (Variables|Default|SetactiveBirdProfileUI 0)
  (CallFunction|DisposeBirdPreview))

(event Custom|DoDownloadBook
  (params (bookId :type String))
  (bind _returnvalue (Utilities|String|MakeLiteralString "{\"uuid\":\"4c52d6b7-51bb-4308-b2a8-d49504f59044\",
\"title\":\"My Private Journal\",\"author\":\"Anonymous\",
\"create_date\":\"2023-06-13T20:42:03.142Z\",
\"testQuote\": \"A wise man once said: \\\"Hello World\\\"\",
\"update_date\":\"2023-06-13T22:31:32.033Z\",
}"))
  (bind _datamap (CallFunction|ParseSimpleJSON _returnvalue))
  ;[0.3327 0.1928 1] Athenaeum
  (bind _keys (Utilities|Map|Keys _datamap))
  (for _array_element _keys
    (Development|PrintString (Utilities|String|Append _array_element " = " (.Value (Utilities|Map|Find _datamap _array_element))) true true "(R=0.000000,G=0.660000,B=1.000000,A=1.000000)" 6.0)))

(event Custom|reqStartPlacement
  (params (itemRef :type Game%20Item%20Ref%20Structure))
  (bind _conancharacter (Utilities|GetConanCharacter))
  ;[0.8878 1 0 0.5] Bird State Manipulation
  (bind _item (CallFunction|ResolveGameItemRef itemRef))
  (bind _asbp_base_bird_item (Utilities|Casting|CastToBP_BaseBirdItem _item))
  (Variables|Default|SetbirdProfileBeingPlaced (Variables|/Game/Mods/RavencrestCouriers/Items/BP_BaseBirdItem.BP_BaseBirdItem_C|GetbirdProfile _asbp_base_bird_item))
  (Default|TriggerStartPlacement _asbp_base_bird_item _conancharacter _conancharacter))

(event Custom|notifyItemBeingPlaced
  (params (item :type Game%20Item%20Ref%20Structure))
  ;[1 0.125 0.125] Document Placeable handling
  (bind _item (CallFunction|ResolveGameItemRef item))
  (bind _templateid (Class|BPRACOIDocument|GetPaperItemTemplateID(Message) _item))
  (Variables|Default|SetdocTemplateID _templateid)
  (bind _document (Class|BPRACOIDocument|GetDocument(Message) _item))
  (Variables|Default|SetdocBeingPlaced _document))

(event Custom|clientOpenBirdProfile2
  (params (profile :type STRUCT%20RACO%20Bird%20Profile%20Structure))
  ;[1 1 1] Bird UI Interaction
  (CallFunction|PrepareBirdPreview (CallFunction|GetBirdTypebyID (Utilities|Struct|BreakSTRUCT_RACO_BirdProfile profile)))
  (bind _windowroot (|GUIModuleControllerActivate (Class|GUIModuleController|GetGUIModuleController) "RACO_ViewBirdProfile" true false)
    (:OnActivate
      (bind _output_get (Variables|Default|SetactiveBirdProfileUI (.AsW%20Bird%20Profile%20View (Utilities|Casting|CastToW_BirdProfile_View _windowroot))))
      (Default|InitUI _output_get profile true)
      (EventDispatchers|BindEventtoSignalClosing _windowroot (delegate Custom|OnBirdProfileUIClosing)))))

(event Custom|OnSignalPlaceBird
  (bind _conancharacter (Utilities|GetConanCharacter))
  ;[1 1 1] Bird UI Interaction
  (CallFunction|ReqStartPlacement (CallFunction|ConstructGameItemRef (stale Custom|OnBirdProfileReceived itemRef)))
  (Default|TriggerStartPlacement (.AsBP%20Base%20Bird%20Item (Utilities|Casting|CastToBP_BaseBirdItem (stale Custom|OnBirdProfileReceived itemRef))) _conancharacter _conancharacter))

(event Custom|OnSignalEquipBird
  ;[1 1 1] Bird UI Interaction
  (CallFunction|ReqEquipBird (CallFunction|ConstructGameItemRef (stale Custom|OnBirdProfileReceived itemRef))))

(event Custom|notifyItemPlacementDone
  (bind _returnvalue (Components|GetOwner))
  (bind _returnvalue_2 (Actor|GetComponentbyClass _returnvalue "/Game/Systems/Building/BP_BuildSystem_v2.BP_BuildSystem_v2_C"))
  ;[1 0.125 0.125] Document Placeable handling
  (if (Variables|/Script/ConanSandbox.BuildSystemComponent|GetIsBuilding _returnvalue_2)
    (Class|BuildSystemComponent|StopBuilding _returnvalue_2)))

(event Custom|reqEquipBird
  (params (itemRef :type Game%20Item%20Ref%20Structure))
  (bind _inventory (Utilities|GetCharacterInventory "ShortcutBar"))
  ;[0.8878 1 0 0.5] Bird State Manipulation
  (bind _item (CallFunction|ResolveGameItemRef itemRef))
  (bind _asbp_base_bird_item (Utilities|Casting|CastToBP_BaseBirdItem _item))
  (if (== _asbp_base_bird_item (Variables|Default|GetequippedBird))
    (Variables|Default|SetequippedBird 0)
    (Variables|Default|SetequippedBirdProfile "")
    (EventDispatchers|UnbindEventfromSignalItemRemoved _inventory (delegate Custom|forceUnequipBird))
    (elif (== (Utilities|GetCharacterInventory "ShortcutBar") (Class|GameItem|GetOwnerInventory _asbp_base_bird_item))
      (bind _output_get (Variables|Default|SetequippedBird _asbp_base_bird_item))
      (Variables|Default|SetequippedBirdProfile (Variables|/Game/Mods/RavencrestCouriers/Items/BP_BaseBirdItem.BP_BaseBirdItem_C|GetbirdProfile _output_get))
      (EventDispatchers|BindEventtoSignalItemRemoved _inventory (delegate Custom|forceUnequipBird)))))

(event Custom|clientOpenBirdDetectionConfig
  (params (birdPlaceable :type BP%20Base%20Bird%20Placeable%20Object%20Reference))
  ;[1 1 1] Bird UI Interaction
  (bind _windowroot (|GUIModuleControllerActivate (Class|GUIModuleController|GetGUIModuleController) "RACO_ViewBirdDetectionConfig" true false)
    (:OnActivate
      (Default|InitUI (.AsW%20Bird%20Detection%20Config%20View (Utilities|Casting|CastToW_BirdDetectionConfig_View _windowroot)) (Variables|/Game/Mods/RavencrestCouriers/Items/BP_BaseBirdPlaceable.BP_BaseBirdPlaceable_C|GetbirdProfile birdPlaceable) (Variables|/Game/Mods/RavencrestCouriers/Items/BP_BaseBirdPlaceable.BP_BaseBirdPlaceable_C|GetbirdDetectionConfig birdPlaceable))
      (EventDispatchers|BindEventtoSignalUpdateConfig (.AsW%20Bird%20Detection%20Config%20View (Utilities|Casting|CastToW_BirdDetectionConfig_View _windowroot)) (delegate Custom|OnSignalUpdateConfig)))))

(event Custom|clientUpdateItemDoc
  (params (item :type Game%20Item%20Ref%20Structure) (document :type STRUCT%20RACO%20Document%20Structure) (triggerCallback :type Boolean))
  ;[1 0.03794 0.3524 0.3] Document client syncing
  (bind _item (CallFunction|ResolveGameItemRef item))
  (Class|BPRACOIDocument|SetDocument(Message) _item document)
  (if triggerCallback
    (CallFunction|ClientDocumentCallback _item document)))

(event Custom|LoopBirdRandomAnimation
  (bind _equippedbirdprofile (Variables|Default|GetequippedBirdProfile))
  (bind _birdtypeid (Utilities|Struct|BreakSTRUCT_RACO_BirdProfile _equippedbirdprofile))
  ;[0.8878 1 0 0.5] Bird State Manipulation
  (if (Math|Boolean|NORBoolean (Networking|IsDedicatedServer) (Utilities|Array|IsEmpty (Utilities|String|ToString(Name) _birdtypeid)))
    (bind _animlength (CallFunction|PlayRandomBirdAnimation (Variables|Default|GetequippedBirdMesh) _birdtypeid))
    (Utilities|FlowControl|Delay (+ _animlength (Math|Random|RandomFloatinRange 2.0 5.0)))
    (CallFunction|LoopBirdRandomAnimation)))

(event Custom|toggleTrackingClient
  ;[0.05805 1 0.1022] Tracking
  (if (Utilities|Struct|BreakSTRUCT_RACO_ServerSettings (CallFunction|GetServerSettings))
    (bind _output_get (Variables|Default|SetisTrackingActive (not (Class|GUIModuleController|IsModuleActive (Class|GUIModuleController|GetGUIModuleController) "RACO_Tracking_HUD"))))
    (bind _returnvalue (Class|GUIModuleController|ActivateModule (Class|GUIModuleController|GetGUIModuleController) "RACO_Tracking_HUD" _output_get false))
    (if (Variables|Default|GetisTrackingActive)
      (bind _outactors (Actor|GetAllActorsOfClass "/Game/Mods/RavencrestCouriers/System/BP_RACO_TrackingSystem.BP_RACO_TrackingSystem_C"))
      (Default|InitHUD (.AsW%20Tracking%20HUD (Utilities|Casting|CastToW_Tracking_HUD _returnvalue)) (Utilities|Array|Get(acopy) _outactors))
      (bind _returnvalue_2 (Utilities|Time|SetTimerbyEvent (delegate Custom|TrackingLoop) 5.0 true))
      (Variables|Default|SettrackingTimer _returnvalue_2)
      (else
        (Utilities|Time|ClearandInvalidateTimerbyHandle (Variables|Default|GettrackingTimer))))
    (else
      (bind _returnvalue_3 (Class|MessageBoxWidget|CreateMessageBox (Components|GetOwner) "OK" "Tracking Disabled" "Bird Tracking has been disabled on this server."))
      (Class|MessageBoxWidget|ShowMessageBox _returnvalue_3 0 1001))))

(event Custom|OnBirdToggleTracking
  ;[1 1 1] Bird UI Interaction
  (CallFunction|ToggleTrackingClient))

(event Custom|OpenDocumentGUIfromPlaceable
  (params (paperObject :type Object%20Object%20Reference) (document :type STRUCT%20RACO%20Document%20Structure))
  ;[0.15 0.15 0.15 0.4] GUI: Document
  (CallFunction|OpenDocumentGUI paperObject (CallFunction|RedactDocument document)))

(event Custom|OnSignalChangeName
  (params (newName :type String))
  ;[1 1 1] Bird UI Interaction
  (EventDispatchers|BindEventtoBirdProfileCallback (delegate Custom|OnBirdNameChanged))
  (CallFunction|ReqChangeBirdName (CallFunction|ConstructGameItemRef (stale Custom|OnBirdProfileReceived itemRef)) newName))

(event Custom|reqGetBirdProfile000
  (params (itemRef :type Game%20Item%20Ref%20Structure))
  ;[0.8878 1 0 0.5] Bird State Manipulation
  (bind _item (CallFunction|ResolveGameItemRef itemRef))
  (bind _asbp_base_bird_item (Utilities|Casting|CastToBP_BaseBirdItem _item))
  (if (CallFunction|IsValidBirdProfile (Variables|/Game/Mods/RavencrestCouriers/Items/BP_BaseBirdItem.BP_BaseBirdItem_C|GetbirdProfile _asbp_base_bird_item))
    (CallFunction|ClientBirdProfileCallback itemRef (Variables|/Game/Mods/RavencrestCouriers/Items/BP_BaseBirdItem.BP_BaseBirdItem_C|GetbirdProfile _asbp_base_bird_item))
    (else
      (bind _newprofile (CallFunction|CreateNewBirdProfile (Variables|/Game/Mods/RavencrestCouriers/Items/BP_BaseBirdItem.BP_BaseBirdItem_C|GetbirdTypeID _asbp_base_bird_item)))
      (bind _output_get (Variables|/Game/Mods/RavencrestCouriers/Items/BP_BaseBirdItem.BP_BaseBirdItem_C|SetbirdProfile _asbp_base_bird_item _newprofile))
      (CallFunction|ClientBirdProfileCallback itemRef _output_get))))

(event Custom|OnBirdProfileReceived
  (params (itemRef :type Game%20Item%20Object%20Reference) (birdProfile :type STRUCT%20RACO%20Bird%20Profile%20Structure))
  ;[1 1 1] Bird UI Interaction
  (EventDispatchers|UnbindEventfromBirdProfileCallback (delegate Custom|OnBirdProfileReceived))
  (CallFunction|PrepareBirdPreview (CallFunction|GetBirdTypebyID (Utilities|Struct|BreakSTRUCT_RACO_BirdProfile birdProfile)))
  (bind _windowroot (|GUIModuleControllerActivate (Class|GUIModuleController|GetGUIModuleController) "RACO_ViewBirdProfile" true false)
    (:OnActivate
      (bind _output_get (Variables|Default|SetactiveBirdProfileUI (.AsW%20Bird%20Profile%20View (Utilities|Casting|CastToW_BirdProfile_View _windowroot))))
      (Default|InitUI _output_get birdProfile false)
      (EventDispatchers|BindEventtoSignalEquipBird (Variables|Default|GetactiveBirdProfileUI) (delegate Custom|OnSignalEquipBird))
      (EventDispatchers|BindEventtoSignalPlaceBird (Variables|Default|GetactiveBirdProfileUI) (delegate Custom|OnSignalPlaceBird))
      (EventDispatchers|BindEventtoSignalChangeBirdName (Variables|Default|GetactiveBirdProfileUI) (delegate Custom|OnSignalChangeName))
      (EventDispatchers|BindEventtoSignalUpdateStats (Variables|Default|GetactiveBirdProfileUI) (delegate Custom|OnSignalUpdateStats))
      (EventDispatchers|BindEventtoSignalClosing (Variables|Default|GetactiveBirdProfileUI) (delegate Custom|OnBirdProfileUIClosing))
      (EventDispatchers|BindEventtoSignalToggleTracking (Variables|Default|GetactiveBirdProfileUI) (delegate Custom|OnBirdToggleTracking)))))

(event Custom|reqChangeBirdName
  (params (itemRef :type Game%20Item%20Ref%20Structure) (newName :type String))
  ;[0.8878 1 0 0.5] Bird State Manipulation
  (bind _item (CallFunction|ResolveGameItemRef itemRef))
  (bind _asbp_base_bird_item (Utilities|Casting|CastToBP_BaseBirdItem _item))
  (bind _structout (Utilities|Struct|SetmembersinSTRUCT_RACO_BirdProfile (Variables|/Game/Mods/RavencrestCouriers/Items/BP_BaseBirdItem.BP_BaseBirdItem_C|GetbirdProfile _asbp_base_bird_item) newName))
  (bind _output_get (Variables|/Game/Mods/RavencrestCouriers/Items/BP_BaseBirdItem.BP_BaseBirdItem_C|SetbirdProfile _asbp_base_bird_item _structout))
  (CallFunction|ClientBirdProfileCallback itemRef _output_get))

(event Custom|reqToggleCanReceive
  (params (endpoint :type Actor%20Component%20Object%20Reference) (canReceive :type Boolean))
  ;[0.15 0.15 0.15 0.4] GUI: Mailbox and Coop
  (Class|BPRACOIMessagingEndpoint|SetCanReceive(Message) endpoint canReceive))

(event Custom|clientDocumentCallback
  (params (paperObject :type Object%20Object%20Reference) (document :type STRUCT%20RACO%20Document%20Structure))
  ;[0.15 0.15 0.15 0.4] Callbacks
  (Default|CallDocumentCallback paperObject document)
  (EventDispatchers|UnbindallEventsfromDocumentCallback))

(event Custom|InitAthenaeumPanel
  (params (panel :type W%20Athenaeum%20Panel%20Object%20Reference))
  ;[0.3327 0.1928 1] Athenaeum
  (EventDispatchers|BindEventtoSignalDownloadBook panel (delegate Custom|DoDownloadBook)))

(event Custom|reqUpdateItemDoc
  (params (item :type Game%20Item%20Object%20Reference))
  ;[1 0.03794 0.3524 0.3] Document client syncing
  ;;[0.15 0.15 0.15 0.5] Is this only needed for short and long item descriptions? (potentially weak reason)
  (bind _asbp_raco_i_document (Utilities|Casting|CastToBP_RACO_I_Document item))
  (bind _document (Default|GetDocument _asbp_raco_i_document))
  (CallFunction|SendDocUpdatetoClient item _document false))

(event Custom|reqDepositItems
  (params (endpoint :type Actor%20Component%20Object%20Reference) (items :type Array%20of%20Game%20Item%20Ref%20Structures))
  ;[0.15 0.15 0.15 0.4] GUI: Mailbox and Coop
  (Class|BPRACOIMessagingEndpoint|DepositItems(Message) endpoint (CallFunction|ResolveGameItemRefArray items)))

(event Custom|reqSaveDocument
  (params (paperItem :type Game%20Item%20Ref%20Structure) (document :type STRUCT%20RACO%20Document%20Structure))
  ;[0.15 0.15 0.15 0.4] GUI: Document
  (bind _item (CallFunction|ResolveGameItemRef paperItem))
  (bind (_success _infomessage) (Class|BPRACOIDocument|TryApplyEdits(Message) _item (Utilities|GetPlayerController) document))
  (Class|ConanCharacter|ClientHUDShowNotification (Utilities|GetConanCharacter) (Utilities|Text|ToText(String) _infomessage) _success true)
  (if _success
    (CallFunction|SendDocUpdatetoClient _item document false)))

(event Custom|InitInventoryDocSync
  (bind _inventory (Utilities|GetCharacterInventory "ShortcutBar"))
  (bind _inventory_2 (Utilities|GetCharacterInventory "Backpack"))
  ;[1 0.03794 0.3524 0.3] Document client syncing
  ;;[0.15 0.15 0.15 0.5] Is this only needed for short and long item descriptions? (potentially weak reason)
  (if (Networking|IsServer)
    (EventDispatchers|BindEventtoSignalItemAdded _inventory_2 (delegate Custom|OnItemAdded))
    (CallFunction|ScanInventoryforDocs _inventory_2)
    (EventDispatchers|BindEventtoSignalItemAdded _inventory (delegate Custom|OnItemAdded))
    (CallFunction|ScanInventoryforDocs _inventory)))

(event Custom|reqPickupBird
  (params (birdPlaceable :type BP%20Base%20Bird%20Placeable%20Object%20Reference))
  (bind _conancharacter (Utilities|GetConanCharacter))
  (bind _returnvalue (Class|ConanCharacter|GetBackpackInventory _conancharacter))
  ;[0.8878 1 0 0.5] Bird State Manipulation
  (Utilities|FlowControl|Sequence
    (:then_0
      (bind _returnvalue_2 (Class|ItemInventory|AddItemTemplate _returnvalue (Variables|/Script/ConanSandbox.BuildableBase|GetSourceItemTemplateID birdPlaceable) -1 "None" 1 false 1.0 -1.0))
      (Variables|/Game/Mods/RavencrestCouriers/Items/BP_BaseBirdItem.BP_BaseBirdItem_C|SetbirdProfile (.AsBP%20Base%20Bird%20Item (Utilities|Casting|CastToBP_BaseBirdItem (Class|ItemInventory|GetItem _returnvalue _returnvalue_2))) (Variables|/Game/Mods/RavencrestCouriers/Items/BP_BaseBirdPlaceable.BP_BaseBirdPlaceable_C|GetbirdProfile birdPlaceable)))
    (:then_1
      (Actor|DestroyActor birdPlaceable))))

(event Custom|reqGetMessagingDestinations
  (params (endpoint :type Actor%20Component%20Object%20Reference))
  ;[0.15 0.15 0.15 0.4] GUI: Mailbox and Coop
  (bind _destinations (Class|BPRACOIMessagingSystem|GetListOfDestinations(Message) (CallFunction|GetMessagingSystem) endpoint))
  (CallFunction|ClientDestinationsCallback _destinations))

(event Custom|OnBirdNameChanged
  (params (itemRef :type Game%20Item%20Object%20Reference) (birdProfile :type STRUCT%20RACO%20Bird%20Profile%20Structure))
  ;[1 1 1] Bird UI Interaction
  (EventDispatchers|UnbindEventfromBirdProfileCallback (delegate Custom|OnBirdNameChanged))
  (Default|InitUI (Variables|Default|GetactiveBirdProfileUI) birdProfile false))

(event Custom|reqNestBird
  (params (nest :type Actor%20Object%20Reference) (bird :type Game%20Item%20Ref%20Structure))
  ;[0.15 0.15 0.15 0.4] GUI: Mailbox and Coop
  (bind _item (CallFunction|ResolveGameItemRef bird))
  (bind (_success _errorinfo) (Class|BPRACOINest|DoNestBird(Message) nest _item))
  (CallFunction|ClientExecutionResultCallback _success _errorinfo))

(event Custom|clientDestinationsCallback
  (params (destinations :type Array%20of%20Strings))
  ;[0.15 0.15 0.15 0.4] Callbacks
  (Default|CallDestinationsCallback destinations)
  (EventDispatchers|UnbindallEventsfromDestinationsCallback))

(event Custom|OnSignalUpdateConfig
  (params (updatedConfig :type STRUCT%20RACO%20Bird%20Detection%20Config%20Structure))
  ;[1 1 1] Bird UI Interaction
  (CallFunction|UpdateBirdDetectionConfig updatedConfig (stale Custom|clientOpenBirdDetectionConfig birdPlaceable)))

(event Custom|reqCopyDocument
  (params (paperItemDest :type Game%20Item%20Ref%20Structure) (document :type STRUCT%20RACO%20Document%20Structure))
  ;[0.15 0.15 0.15 0.4] GUI: Document
  (bind _item (CallFunction|ResolveGameItemRef paperItemDest))
  (bind (_success _infomessage) (Class|BPRACOIDocument|TryMakeCopy(Message) _item (Utilities|GetPlayerController) document))
  (Class|ConanCharacter|ClientHUDShowNotification (Utilities|GetConanCharacter) (Utilities|Text|ToText(String) _infomessage) _success true)
  (if _success
    (CallFunction|SendDocUpdatetoClient _item document false)))

(event Custom|reqBreakSeal
  (params (itemRef :type Game%20Item%20Ref%20Structure))
  ;[0.15 0.15 0.15 0.4] GUI: Document
  (bind _item (CallFunction|ResolveGameItemRef itemRef))
  (bind (_success _infomessage) (Class|BPRACOIDocument|TryBreakSeal(Message) _item))
  (Class|ConanCharacter|ClientHUDShowNotification (Utilities|GetConanCharacter) (Utilities|Text|ToText(String) _infomessage) _success true)
  (if _success
    (bind _document (Class|BPRACOIDocument|GetDocument(Message) _item))
    (CallFunction|SendDocUpdatetoClient _item _document true)))

(event Custom|OnItemAdded
  (params (index :type Integer) (item :type Game%20Item%20Object%20Reference) (srcInventory :type Item%20Inventory%20Object%20Reference) (srcIndex :type Integer))
  ;[1 0.03794 0.3524 0.3] Document client syncing
  ;;[0.15 0.15 0.15 0.5] Is this only needed for short and long item descriptions? (potentially weak reason)
  (CallFunction|ReqUpdateItemDoc item))

(event EventBeginPlay
  (if (Networking|IsServer)
    ;[0.15 0.15 0.15 0.5] Why is this needed?
    (CallFunction|InitInventoryDocSync)
    (else
      (CallFunction|OnRepEquippedBirdProfile))))

(fn PrepareBirdPreview
  (params (birdType :type STRUCT%20RACO%20Bird%20Type%20Structure))
  (bind (_skeletalmesh _transform _idleanimations) (Utilities|Struct|BreakSTRUCT_RACO_BirdType birdType))
  (Utilities|FlowControl|Sequence
    (:then_0
      (Utilities|IsValid (Variables|Default|GetbirdPreviewRoom)
        (:Is%20Not%20Valid
          (bind _returnvalue (Game|SpawnActorfromClass "/Game/Mods/RavencrestCouriers/UI/bird_preview/BP_RACO_PreviewRoom.BP_RACO_PreviewRoom_C" (Math|Conversions|ToTransform(Vector) "0, 0,-15000.000000") "Undefined" "OverrideRootScale" (Components|GetOwner) 0))
          (Variables|Default|SetbirdPreviewRoom _returnvalue))))
    (:then_1
      (Transformation|SetRelativeTransform (Variables|/Game/Mods/RavencrestCouriers/UI/bird_preview/BP_RACO_PreviewRoom.BP_RACO_PreviewRoom_C|GetSkeletalMesh (Variables|Default|GetbirdPreviewRoom)) _transform false false)
      (Components|SkinnedMesh|SetSkinnedAssetandUpdate (Variables|/Game/Mods/RavencrestCouriers/UI/bird_preview/BP_RACO_PreviewRoom.BP_RACO_PreviewRoom_C|GetSkeletalMesh (Variables|Default|GetbirdPreviewRoom)) _skeletalmesh true)
      (Components|Animation|PlayAnimation (Variables|/Game/Mods/RavencrestCouriers/UI/bird_preview/BP_RACO_PreviewRoom.BP_RACO_PreviewRoom_C|GetSkeletalMesh (Variables|Default|GetbirdPreviewRoom)) (Utilities|Array|Get(acopy) _idleanimations) true))))

(fn OnRepEquippedBirdProfile
  (bind _equippedbirdprofile (Variables|Default|GetequippedBirdProfile))
  (bind _birdtypeid (Utilities|Struct|BreakSTRUCT_RACO_BirdProfile _equippedbirdprofile))
  (bind _birdtype (CallFunction|GetBirdTypebyID _birdtypeid))
  (bind (_skeletalmesh _transform) (Utilities|Struct|BreakSTRUCT_RACO_BirdType _birdtype))
  (Utilities|FlowControl|Sequence
    (:then_0
      (bind _output_get (LocalVariables|Setcharacter (Utilities|GetConanCharacter)))
      (Utilities|IsValid _output_get
        (:Is%20Valid
          (LocalVariables|SetcharacterGender (Class|ConanCharacter|GetIntStat _output_get "Gender" "Full")))))
    (:then_1
      (Utilities|IsValid (Variables|Default|GetequippedBirdMesh)
        (:Is%20Not%20Valid
          (bind _returnvalue (Class|CharacterFunctionLibrary|AddSkeletalMeshComponent (LocalVariables|Getcharacter) true (Utilities|Select :Index (- (LocalVariables|GetcharacterGender) 1) :Option%200 (LocalVariables|GetmaleTransform) :Option%201 (LocalVariables|GetfemaleTransform)) "/Script/Engine.SkeletalMeshComponent"))
          (bind _output_get_2 (Variables|Default|SetequippedBirdMesh _returnvalue))
          (Transformation|AttachComponentToComponent _output_get_2 (Variables|/Script/Engine.Character|GetMesh (LocalVariables|Getcharacter)) "b_R_clavicle" "KeepRelative" "KeepRelative" "KeepRelative" true))))
    (:then_2
      (if (CallFunction|IsValidBirdProfile _equippedbirdprofile)
        (Transformation|SetRelativeTransform (Variables|Default|GetequippedBirdMesh) (Math|Transform|ComposeTransforms (Utilities|Select :Index (- (LocalVariables|GetcharacterGender) 1) :Option%200 (LocalVariables|GetmaleTransform) :Option%201 (LocalVariables|GetfemaleTransform)) _transform) false false)
        (Components|SkinnedMesh|SetSkinnedAssetandUpdate (Variables|Default|GetequippedBirdMesh) _skeletalmesh true)
        (CallFunction|LoopBirdRandomAnimation)
        (else
          (Components|SkinnedMesh|SetSkinnedAssetandUpdate (Variables|Default|GetequippedBirdMesh) 0 true))))))

(fn IsBirdEquipped
  (params (profileGUID :type String))
  (return (Utilities|Enum|Equal(Enum) profileGUID (Utilities|Struct|BreakSTRUCT_RACO_BirdProfile (Variables|Default|GetequippedBirdProfile)))))

(fn DisposeBirdPreview
  (Utilities|IsValid (Variables|Default|GetbirdPreviewRoom)
    (:Is%20Valid
      (Actor|DestroyActor (Variables|Default|GetbirdPreviewRoom))
      (Variables|Default|SetbirdPreviewRoom 0))))

(fn RedactDocument
  (params (document :type STRUCT%20RACO%20Document%20Structure))
  (Utilities|FlowControl|Sequence
    (:then_0
      (if (.sealed (Utilities|Struct|BreakSTRUCT_RACO_Document document))
        (bind _output_get (LocalVariables|SetlocalDocument document))
        (bind _structout (Utilities|Struct|SetmembersinSTRUCT_RACO_Document _output_get (Utilities|Array|MakeArray)))
        (return _structout)))
    (:then_1
      (return document))))

(fn SendDocUpdatetoClient
  (params (item :type Game%20Item%20Object%20Reference) (document :type STRUCT%20RACO%20Document%20Structure) (triggerCallback :type Boolean))
  (CallFunction|ClientUpdateItemDoc (CallFunction|ConstructGameItemRef item) (CallFunction|RedactDocument document) triggerCallback))