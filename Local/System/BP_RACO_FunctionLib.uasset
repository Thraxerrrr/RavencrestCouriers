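; Blueprint function library for the RACO system, with shared helpers for written documents, messenger birds and game item references.
; Document helpers handle IDs, pages, descriptions and splitting image URLs out of text; item refs store inventory plus index for later resolution and weight checks.
; Bird helpers build profiles and derive speed, carry weight and detection range from type and levelling DataTables.
; Other utilities locate system actors, play attenuated sounds and look up XP thresholds.
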(fn GenerateDocID
  (return (Guid|ToString(Guid) (Guid|NewGuid))))

(fn IsValidGUID
  (params (docID :type String))
  (return (> (Utilities|String|Len docID) 0)))

(fn ConstructGameItemRef
  (params (gameItem :type Game%20Item%20Object%20Reference))
  (bind _returnvalue (Class|GameItem|GetOwnerInventory gameItem))
  (return (Utilities|Struct|MakeGameItemRef _returnvalue (Class|ItemInventory|GetItemIndex _returnvalue gameItem))))

(fn ConstructBlankDocument
  (return (Utilities|Struct|MakeSTRUCT_RACO_Document "" false "" "" "" "" (Utilities|Array|MakeArray))))

(fn ParseImagesinText
  (params (text :type String))
  (bind _textblocks (LocalVariables|GettextBlocks))
  (bind _output_get (LocalVariables|SettextInput text))
  (LocalVariables|SettextLength (Utilities|String|Len _output_get))
  ;[1 1 1] Loop until end of text
  (while (< (LocalVariables|GetcurrentPos) (LocalVariables|GettextLength))
    ;[1 1 1] Search for next hyperlink
    (if (== (Utilities|String|FindSubstring (LocalVariables|GettextInput) "http" false false (LocalVariables|GetcurrentPos)) -1)
      (LocalVariables|Setmark (LocalVariables|GetcurrentPos))
      (LocalVariables|SetcurrentPos (LocalVariables|GettextLength))
      ;[1 1 1] Copy block of text to output array
      (Utilities|Array|Add _textblocks (Utilities|String|GetSubstring (LocalVariables|GettextInput) (LocalVariables|Getmark) (- (LocalVariables|GetcurrentPos) (LocalVariables|Getmark))))
      (else
        (LocalVariables|Setmark (LocalVariables|GetcurrentPos))
        (LocalVariables|SetcurrentPos (Utilities|String|FindSubstring (LocalVariables|GettextInput) "http" false false (LocalVariables|GetcurrentPos)))
        (Utilities|Array|Add _textblocks (Utilities|String|GetSubstring (LocalVariables|GettextInput) (LocalVariables|Getmark) (- (LocalVariables|GetcurrentPos) (LocalVariables|Getmark))))
        ;[1 1 1] Search for end of hyperlink (line break or whitespace)
        (if (and (== (Utilities|String|FindSubstring (LocalVariables|GettextInput) "
" false false (LocalVariables|GetcurrentPos)) -1) (== (Utilities|String|FindSubstring (LocalVariables|GettextInput) " " false false (LocalVariables|GetcurrentPos)) -1))
          ;[1 1 1] Hyperlink goes to end of text
          (LocalVariables|Setmark (LocalVariables|GetcurrentPos))
          (LocalVariables|SetcurrentPos (LocalVariables|GettextLength))
          (else
            ;[1 1 1] Hyperlink ends with line break or whitespace
            (LocalVariables|Setmark (LocalVariables|GetcurrentPos))
            (LocalVariables|SetcurrentPos (CallFunction|GetSmallestPositive (Utilities|String|FindSubstring (LocalVariables|GettextInput) "
" false false (LocalVariables|GetcurrentPos)) (Utilities|String|FindSubstring (LocalVariables|GettextInput) " " false false (LocalVariables|GetcurrentPos))))))
        ;[1 1 1] Append hyperlink to imageURL array
        (Utilities|Array|Add (LocalVariables|GetimageURLs) (Utilities|String|GetSubstring (LocalVariables|GettextInput) (LocalVariables|Getmark) (- (LocalVariables|GetcurrentPos) (LocalVariables|Getmark)))))))
  (return (LocalVariables|GettextBlocks) (LocalVariables|GetimageURLs)))

(fn ResolveGameItemRef
  (params (itemRef :type Game%20Item%20Ref%20Structure))
  (bind (_inventory _itemindex) (Utilities|Struct|BreakGameItemRef itemRef))
  (return (Class|ItemInventory|GetItem _inventory _itemindex)))

(fn IsNewDocument
  (params (document :type STRUCT%20RACO%20Document%20Structure))
  (return (not (CallFunction|IsValidGUID (Utilities|Struct|BreakSTRUCT_RACO_Document document)))))

(fn UpdateDocumentPages
  (params (pages :type Map%20of%20Integers%20to%20Strings) (document :type STRUCT%20RACO%20Document%20Structure))
  (bind _keys (Utilities|Map|Keys pages))
  (LocalVariables|SetpageCount (Utilities|Array|Length _keys))
  (LocalVariables|SetcurrentPage 1)
  (while (<= (LocalVariables|GetcurrentPage) (LocalVariables|GetpageCount))
    (Utilities|Array|Add (LocalVariables|GettextPages) (.Value (Utilities|Map|Find pages (LocalVariables|GetcurrentPage))))
    (Math|Integer|IncrementInt (LocalVariables|GetcurrentPage)))
  (bind _structout (Utilities|Struct|SetmembersinSTRUCT_RACO_Document document (LocalVariables|GettextPages)))
  (return _structout))

(fn GetDocumentDescription
  (params (document :type STRUCT%20RACO%20Document%20Structure) (short :type Boolean))
  (LocalVariables|SetshortDesc short)
  (bind _output_get (LocalVariables|Setdoc document))
  ;[1 1 1] Empty docs
  (if (> (Utilities|String|Len (Utilities|Struct|BreakSTRUCT_RACO_Document _output_get)) 0)
    (Utilities|FlowControl|Sequence
      (:then_0
        ;[1 1 1] Sealed docs
        (if (.sealed (Utilities|Struct|BreakSTRUCT_RACO_Document (LocalVariables|Getdoc)))
          (if (== (Utilities|String|Len (.sealName (Utilities|Struct|BreakSTRUCT_RACO_Document (LocalVariables|Getdoc)))) 0)
            (LocalVariables|SetoutputStringBuffer "A sealed document.")
            (else
              (LocalVariables|SetoutputStringBuffer (Utilities|String|Append "A document, sealed by \"" (.sealName (Utilities|Struct|BreakSTRUCT_RACO_Document (LocalVariables|Getdoc))) "\""))))
          (return (LocalVariables|GetoutputStringBuffer))))
      (:then_1
        ;[1 1 1] Append title, if any
        (if (> (Utilities|String|Len (Utilities|Struct|BreakSTRUCT_RACO_Document (LocalVariables|Getdoc))) 0)
          (LocalVariables|SetoutputStringBuffer (Utilities|String|Append "\"" (Utilities|Struct|BreakSTRUCT_RACO_Document (LocalVariables|Getdoc)) "\""))
          ;[1 1 1] Append author, if any
          (if (> (Utilities|String|Len (Utilities|Struct|BreakSTRUCT_RACO_Document (LocalVariables|Getdoc))) 0)
            (LocalVariables|SetoutputStringBuffer (Utilities|String|Append (LocalVariables|GetoutputStringBuffer) ", by " (Utilities|Struct|BreakSTRUCT_RACO_Document (LocalVariables|Getdoc)) "
")))))
      (:then_2
        ;[1 1 1] Append a bit of the text
        (if (LocalVariables|GetshortDesc)
          (LocalVariables|SettextLengthToAppend 20)
          (else
            (LocalVariables|SettextLengthToAppend 300)))
        (LocalVariables|SetoutputStringBuffer (Utilities|String|Append (LocalVariables|GetoutputStringBuffer) "\"" (Utilities|String|GetSubstring (Utilities|Array|Get(acopy) (Utilities|Struct|BreakSTRUCT_RACO_Document (LocalVariables|Getdoc))) 0 (LocalVariables|GettextLengthToAppend))))
        (if (> (Utilities|String|Len (Utilities|Array|Get(acopy) (Utilities|Struct|BreakSTRUCT_RACO_Document (LocalVariables|Getdoc)))) (LocalVariables|GettextLengthToAppend))
          (LocalVariables|SetoutputStringBuffer (Utilities|String|Append (LocalVariables|GetoutputStringBuffer) "...")))
        (LocalVariables|SetoutputStringBuffer (Utilities|String|Append (LocalVariables|GetoutputStringBuffer) "\"")))
      (:then_3
        (return (LocalVariables|GetoutputStringBuffer))))
    (else
      (return "A document."))))

(fn DoctoString
  (params (doc :type STRUCT%20RACO%20Document%20Structure))
  (bind (_documentid _sealed _sealname _sealimageurl _title _author _text) (Utilities|Struct|BreakSTRUCT_RACO_Document doc))
  (return (Utilities|String|Append "Doc [id: " _documentid "][sealed: " (Utilities|String|ToString(Boolean) _sealed) "][title: " _title "][author: " _author "][pagecount: " (Utilities|String|ToString(Integer) (Utilities|Array|Length _text)) "], page1: " (Utilities|Array|Get(acopy) _text))))

(fn GetInventoryViewSelectedIndex
  (params (inventoryView :type Inventory%20View%20Object%20Reference))
  (bind _itemgridview (Variables|/Game/UI/Inventory/InventoryView.InventoryView_C|GetItemGridView inventoryView))
  (bind _scrollbox (Variables|/Game/UI/Framework/InventoryGridView.InventoryGridView_C|GetScrollBox _itemgridview))
  (bind _returnvalue (Class|PanelWidget|GetChildat _scrollbox))
  (bind _assize_box (Utilities|Casting|CastToSizeBox _returnvalue))
  (bind _returnvalue_2 (Class|PanelWidget|GetChildat _assize_box))
  (bind _aspanel_widget (Utilities|Casting|CastToPanelWidget _returnvalue_2))
  (while (< (LocalVariables|Getindex) (Class|PanelWidget|GetChildrenCount _aspanel_widget))
    (if (>= (Utilities|Struct|BreakLinearColor (Variables|/Script/UMG.Border|GetBrushColor (.AsBorder (Utilities|Casting|CastToBorder (Class|PanelWidget|GetChildat (Widget|GetParent (Variables|/Game/UI/Framework/InventoryGridSlotView.InventoryGridSlotView_C|GetSlotImage (.AsInventory%20Grid%20Slot%20View (Utilities|Casting|CastToInventoryGridSlotView (Class|PanelWidget|GetChildat _aspanel_widget (LocalVariables|Getindex)))))) 2))))) 0.5)
      (return (LocalVariables|Getindex))
      (else
        (Math|Integer|IncrementInt (LocalVariables|Getindex)))))
  (return -1))

(fn ResolveGameItemRefDocs
  (params (itemRefs :type Array%20of%20Game%20Item%20Ref%20Structures))
  (for _array_element itemRefs
    (bind _item (CallFunction|ResolveGameItemRef _array_element))
    (bind _asbp_base_document_item (Utilities|Casting|CastToBP_BaseDocumentItem _item))
    (Utilities|Array|Add (LocalVariables|GettmpItemIDs) (Variables|/Script/ConanSandbox.GameItem|GetTemplateID _asbp_base_document_item))
    (Utilities|Array|Add (LocalVariables|GettmpDocs) (Variables|/Game/Mods/RavencrestCouriers/Items/BP_BaseDocumentItem.BP_BaseDocumentItem_C|Getdocument _asbp_base_document_item)))
  (return (LocalVariables|GettmpItemIDs) (LocalVariables|GettmpDocs)))

(fn HasTimePassed
  (params (startTime :type Date%20Time%20Structure) (seconds :type Integer))
  (return (< (+ startTime (Math|Timespan|MakeTimespan 0 0 0 seconds)) (Math|DateTime|Now))))

(fn GetBirdDefaultObject
  (params (birdTemplateID :type Integer))
  (bind _returnvalue (Utilities|GetDataTableRow "/Game/Items/ItemTable.ItemTable" (Utilities|String|StringToName (Utilities|String|ToString(Integer) birdTemplateID)))
    (:then
      (bind _asbp_base_bird_item (Utilities|Casting|CastToBP_BaseBirdItem (Class|DreamworldBlueprints|GetClassDefaultObject (Utilities|ResolveSoftReference (.ItemClass (Utilities|Struct|BreakItemTableRow _returnvalue)))))
        (:then
          (return _asbp_base_bird_item))
        (:CastFailed
          (return 0))))
    (:RowNotFound
      (return 0))))

(fn GetSmallestPositive
  (params (n1 :type Integer) (n2 :type Integer))
  (bind _returnvalue (>= n2 0))
  (bind _returnvalue_2 (>= n1 0))
  (Utilities|And+Branch _returnvalue_2 _returnvalue
    (:True
      ;[1 1 1] Both are positive: return the smallest
      (return (Math|Integer|Min(Integer) n1 n2)))
    (:False
      (Utilities|And+Branch (not _returnvalue_2) (not _returnvalue)
        (:True
          ;[1 1 1] Both are negative: return -1
          (return -1))
        (:False
          ;[1 1 1] One is negative: return the positive one
          (return (Math|Integer|Max(Integer) n1 n2)))))))

(fn IsBird
  (params (item :type Game%20Item%20Object%20Reference))
  (return (Utilities|ClassIsChildOf (Utilities|GetClass item) "/Game/Mods/RavencrestCouriers/Items/BP_BaseBirdItem.BP_BaseBirdItem_C")))

(fn GetServerSettings
  (return (Variables|/Game/Mods/RavencrestCouriers/System/BP_RACO_SettingsSystem.BP_RACO_SettingsSystem_C|GetserverSettings (CallFunction|GetSettingsSystem))))

(fn GetSettingsSystem
  (bind _outactors (Actor|GetAllActorsOfClass 0 "/Game/Mods/RavencrestCouriers/System/BP_RACO_SettingsSystem.BP_RACO_SettingsSystem_C"))
  (return (Utilities|Array|Get(acopy) _outactors)))

(fn GetMessagingSystem
  (bind _outactors (Actor|GetAllActorsOfClass 0 "/Game/Mods/RavencrestCouriers/System/BP_RACO_MessagingSystem.BP_RACO_MessagingSystem_C"))
  (return (Utilities|Array|Get(acopy) _outactors)))

(fn GetBirdTypefromTemplateID
  (params (templateID :type Integer))
  (bind _bird (CallFunction|GetBirdDefaultObject templateID))
  (return (CallFunction|GetBirdTypebyID (Variables|/Game/Mods/RavencrestCouriers/Items/BP_BaseBirdItem.BP_BaseBirdItem_C|GetbirdTypeID _bird))))

(fn CreateNewBirdProfile
  (params (birdTypeID :type String))
  (bind _returnvalue (Utilities|GetDataTableRow "/Game/Mods/RavencrestCouriers/System/DT_RACO_BirdTypes.DT_RACO_BirdTypes" (Utilities|String|StringToName birdTypeID))
    (:then
      (return (Utilities|Struct|MakeSTRUCT_RACO_BirdProfile (.name (Utilities|Struct|BreakSTRUCT_RACO_BirdType _returnvalue)) birdTypeID (Math|Random|RandomIntegerinRange 0 1) 0 0 (.baseColor (Utilities|Struct|BreakSTRUCT_RACO_BirdType _returnvalue)) 0 0 0 0 (Guid|ToString(Guid) (Guid|NewGuid)))))
    (:RowNotFound
      (return ""))))

(fn IsValidBirdProfile
  (params (birdProfile :type STRUCT%20RACO%20Bird%20Profile%20Structure))
  (return (> (Utilities|String|Len (Utilities|Struct|BreakSTRUCT_RACO_BirdProfile birdProfile)) 0)))

(fn GetBirdTypebyID
  (params (birdTypeID :type String))
  (bind _returnvalue (Utilities|GetDataTableRow "/Game/Mods/RavencrestCouriers/System/DT_RACO_BirdTypes.DT_RACO_BirdTypes" (Utilities|String|StringToName birdTypeID))
    (:then
      (return _returnvalue))
    (:RowNotFound
      (return ""))))

(fn CalcBirdTravelSpeed
  (params (birdProfile :type STRUCT%20RACO%20Bird%20Profile%20Structure))
  (bind (_birdtypeid _travelspeedpoints) (Utilities|Struct|BreakSTRUCT_RACO_BirdProfile birdProfile))
  (bind _birdtype (CallFunction|GetBirdTypebyID _birdtypeid))
  (bind _basetravelspeed (Utilities|Struct|BreakSTRUCT_RACO_BirdType _birdtype))
  (bind _returnvalue (Utilities|GetDataTableRow "/Game/Mods/RavencrestCouriers/System/DT_RACO_BirdTypeLevelling.DT_RACO_BirdTypeLevelling" (Utilities|String|StringToName _birdtypeid))
    (:then
      (return (+ (* (.speedIncrementPerPoint (Utilities|Struct|BreakSTRUCT_RACO_BirdTypeLevelling _returnvalue)) (Math|Conversions|ToFloat(Integer) _travelspeedpoints)) _basetravelspeed)))
    (:RowNotFound
      (return _basetravelspeed))))

(fn CalcBirdCarryWeight
  (params (birdProfile :type STRUCT%20RACO%20Bird%20Profile%20Structure))
  (bind (_birdtypeid _carryweightpoints) (Utilities|Struct|BreakSTRUCT_RACO_BirdProfile birdProfile))
  (bind _birdtype (CallFunction|GetBirdTypebyID _birdtypeid))
  (bind _basecarryweight (Utilities|Struct|BreakSTRUCT_RACO_BirdType _birdtype))
  (bind _returnvalue (Utilities|GetDataTableRow "/Game/Mods/RavencrestCouriers/System/DT_RACO_BirdTypeLevelling.DT_RACO_BirdTypeLevelling" (Utilities|String|StringToName _birdtypeid))
    (:then
      (return (+ (* (.weightIncrementPerPoint (Utilities|Struct|BreakSTRUCT_RACO_BirdTypeLevelling _returnvalue)) (Math|Conversions|ToFloat(Integer) _carryweightpoints)) _basecarryweight)))
    (:RowNotFound
      (return _basecarryweight))))

(fn CalcBirdDetectionRange
  (params (birdProfile :type STRUCT%20RACO%20Bird%20Profile%20Structure))
  (bind (_birdtypeid _detectionrangepoints) (Utilities|Struct|BreakSTRUCT_RACO_BirdProfile birdProfile))
  (bind _birdtype (CallFunction|GetBirdTypebyID _birdtypeid))
  (bind _basedetectionrange (Utilities|Struct|BreakSTRUCT_RACO_BirdType _birdtype))
  (bind _returnvalue (Utilities|GetDataTableRow "/Game/Mods/RavencrestCouriers/System/DT_RACO_BirdTypeLevelling.DT_RACO_BirdTypeLevelling" (Utilities|String|StringToName _birdtypeid))
    (:then
      (return (+ (* (.detectionIncrementPerPoint (Utilities|Struct|BreakSTRUCT_RACO_BirdTypeLevelling _returnvalue)) (Math|Conversions|ToFloat(Integer) _detectionrangepoints)) _basedetectionrange)))
    (:RowNotFound
      (return _basedetectionrange))))

(fn IsItemBelowWeight
  (params (itemRef :type Game%20Item%20Ref%20Structure) (availableWeight :type Float%20%28single-precision%29))
  (bind _item (CallFunction|ResolveGameItemRef itemRef))
  (bind _returnvalue (Utilities|GetDataTableRow "/Game/Items/ItemTable.ItemTable" (Utilities|String|StringToName (Utilities|String|ToString(Integer) (Variables|/Script/ConanSandbox.GameItem|GetTemplateID _item))))
    (:then
      (return (<= (* (Class|GameItem|GetIntStat _item "StackSize") (.EncumbranceWeight (Utilities|Struct|BreakItemTableRow _returnvalue))) availableWeight)))
    (:RowNotFound
      (return false))))

(fn GetTotalItemsWeight
  (params (itemRefs :type Array%20of%20Game%20Item%20Ref%20Structures))
  (for _array_element itemRefs
    (bind _item (CallFunction|ResolveGameItemRef _array_element))
    (bind _returnvalue (Utilities|GetDataTableRow "/Game/Items/ItemTable.ItemTable" (Utilities|String|StringToName (Utilities|String|ToString(Integer) (Variables|/Script/ConanSandbox.GameItem|GetTemplateID _item))))
      (:then
        (LocalVariables|SetweightSum (+ (LocalVariables|GetweightSum) (* (Class|GameItem|GetIntStat _item "StackSize") (.EncumbranceWeight (Utilities|Struct|BreakItemTableRow _returnvalue))))))))
  (return (LocalVariables|GetweightSum)))

(fn PlaySoundat
  (params (audioComponent :type Conan%20Audio%20Component%20Object%20Reference) (sound :type Sound%20Base%20Object%20Reference))
  (if (|IsAssetValid sound)
    (bind _returnvalue (Class|FuncomGenericLibrary|SyncLoadAsset sound))
    (Class|ConanAudioComponent|SetSound audioComponent (.AsSound%20Base (Utilities|Casting|CastToSoundBase _returnvalue)))
    (bind _outactors (Actor|GetAllActorsOfClass 0 "/Game/Systems/BP_ServerSettings.BP_ServerSettings_C"))
    (Variables|/Script/ConanSandbox.ConanAudioComponent|SetbOverrideAttenuation audioComponent true)
    (Variables|/Script/ConanSandbox.ConanAudioComponent|SetAttenuationOverrides audioComponent (Utilities|Struct|MakeSoundAttenuationSettings true true "Linear" "Sphere" -6e+01 "0.000000,0.000000,0.000000" (Math|Float|Max(Float) (Variables|/Script/ConanSandbox.ServerSettings|GetChatLocalRadius (Utilities|Array|Get(acopy) _outactors)) 5e+02)))
    (Class|ConanAudioComponent|Play audioComponent 0.0)))

(fn GetExperienceSystem
  (bind _outactors (Actor|GetAllActorsOfClass 0 "/Game/Mods/RavencrestCouriers/System/BP_RACO_ExperienceSystem.BP_RACO_ExperienceSystem_C"))
  (return (Utilities|Array|Get(acopy) _outactors)))

(fn GetXPRequiredforLevel
  (params (targetLevel :type Integer))
  (LocalVariables|Setlevel targetLevel)
  (bind _outrownames (DataTable|GetDataTableRowNames "/Game/Systems/Thrall/NPCLevelCurveDataTable.NPCLevelCurveDataTable"))
  (for _array_element _outrownames
    (bind _returnvalue (Utilities|GetDataTableRow "/Game/Systems/Thrall/NPCLevelCurveDataTable.NPCLevelCurveDataTable" _array_element)
      (:then
        (if (and (Utilities|Name|Equal(Name) (.CurveName (Utilities|Struct|BreakNPCProgressionCurveRow _returnvalue)) "Normal") (== (+ (.Level (Utilities|Struct|BreakNPCProgressionCurveRow _returnvalue)) 1) (LocalVariables|Getlevel)))
          (LocalVariables|Setxp (.XPRequired (Utilities|Struct|BreakNPCProgressionCurveRow _returnvalue)))))))
  (return (LocalVariables|Getxp)))