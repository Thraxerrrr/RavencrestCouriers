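; Actor component that makes a buildable an endpoint for sending and receiving item messages carried by bird couriers.
; On the server it registers with the messaging system, retrying until available, and unregisters on EndPlay.
; Validated sends move items into transit; receivers get the payload without the bird, which returns to a sending nest on delivery notification.
; Bird sounds multicast at each stage, and a persisted flag controls whether it is listed as a destination.
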(event Custom|handleMessageDeliveredNotification
  (params (message :type STRUCT%20RACO%20Message%20in%20Flight%20Structure))
  (bind (_birdtemplateid _itemtransitslots) (Utilities|Struct|BreakSTRUCT_RACO_MessageInFlight message))
  (bind _returnvalue (Components|GetOwner))
  ;[1 1 1] A message sent from this endpoint has reached its destination
  (CallFunction|MulticastPlayBirdSound _birdtemplateid)
  (if (CallFunction|HasNest _returnvalue)
    (bind _hasfreeslots (Class|BPRACOINest|HasFreeNestingSlots(Message) _returnvalue))
    (Class|BPRACOIMessagingSystem|MoveItemfromTransit(Message) (Utilities|GetMessagingSystem) (Utilities|Array|Get(acopy) _itemtransitslots) (Utilities|GetOwnerInventory (select _hasfreeslots "PetInventory" "PlaceableInventory")))))

(event Custom|DoReceiveMessage
  (params (message :type STRUCT%20RACO%20Message%20in%20Flight%20Structure))
  (bind (_birdtemplateid _itemtransitslots) (Utilities|Struct|BreakSTRUCT_RACO_MessageInFlight message))
  ;[1 1 1] Receive a message
  (bind (_array_element _array_index) (Utilities|ForEachLoopFast _itemtransitslots)
    (:LoopBody
      ;;[1 1 1] Skip first item: the bird
      (if (> _array_index 0)
        (Class|BPRACOIMessagingSystem|MoveItemfromTransit(Message) (Utilities|GetMessagingSystem) _array_element (Utilities|GetOwnerInventory "PlaceableInventory"))))
    (:Completed
      (CallFunction|MulticastPlayBirdSound _birdtemplateid))))

(event Custom|multicastPlayBirdSound
  (params (courierID :type Integer))
  (if (not (Networking|IsDedicatedServer))
    (bind _birdtype (CallFunction|GetBirdTypefromTemplateID courierID))
    (CallFunction|PlayBirdSound (Variables|Default|GetaudioComponent) _birdtype)))

(event Custom|TryInit
  ;[1 1 1] Wait until MessagingSystem is available
  (Utilities|IsValid (Utilities|GetMessagingSystem)
    (:Is%20Valid
      ;[1 1 1] Register/unregister this messaging endpoint in the messaging system
      (Class|BPRACOIMessagingSystem|RegisterEndpoint(Message) (Utilities|GetMessagingSystem) self))
    (:Is%20Not%20Valid
      (Utilities|Time|SetTimerbyEvent (delegate Custom|TryInit) 1.0))))

(event EventEndPlay
  (params (EndPlayReason :type EEndPlayReason%20Enum :default "Destroyed"))
  ;[1 1 1] Register/unregister this messaging endpoint in the messaging system
  (if (Networking|IsServer)
    (if (not (CallFunction|IsABrush (Components|GetOwner)))
      (Class|BPRACOIMessagingSystem|UnregisterEndpoint(Message) (Utilities|GetMessagingSystem) self))))

(event EventBeginPlay
  (if (Networking|IsServer)
    (if (not (CallFunction|IsABrush (Components|GetOwner)))
      ;[1 1 1] Wait until MessagingSystem is available
      (Utilities|Time|SetTimerbyEvent (delegate Custom|TryInit) 1.0))))

(fn GetDisplayName
  (bind _returnvalue (Components|GetOwner))
  (bind _asbuildable_base (Utilities|Casting|CastToBuildableBase _returnvalue))
  (bind _returnvalue_2 (Class|BuildableBase|GetOwnerName _asbuildable_base))
  (return (Utilities|String|Append (Utilities|String|ToString(Text) _returnvalue_2) " (" (Utilities|String|ToString(Text) (Class|BuildableBase|GetBuildableName _asbuildable_base false)) ")")))

(fn GetUniqueID
  (return (Class|DreamworldBlueprints|ToString(UniqueID) (Class|UniqueID|GetActorUID (Components|GetOwner)))))

(fn DoDepositItems
  (params (items :type Array%20of%20Game%20Item%20Object%20References))
  (LocalVariables|SetlocalInventory (Utilities|GetOwnerInventory "PlaceableInventory"))
  (bind _array_element (Utilities|ForEachLoopFast items)
    (:LoopBody
      (Class|ItemInventory|MoveItem (.inventory (CallFunction|GetPlacementinInventory _array_element)) (.slot (CallFunction|GetPlacementinInventory _array_element)) (LocalVariables|GetlocalInventory) -1 -1 false))))

(fn GetCanReceive
  (return (Variables|Default|GetcanReceive)))

(fn SerializeDestination
  (params (destinations :type Array%20of%20Strings))
  (if (Variables|Default|GetcanReceive)
    (bind _name (CallFunction|GetDisplayName))
    (Utilities|Array|Add destinations (CallFunction|MakeEndpointString _name (CallFunction|GetUniqueID)))))

(fn SetCanReceive
  (params (canReceiveMessages :type Boolean))
  (Variables|Default|SetcanReceive canReceiveMessages)
  (Class|PersistenceComponent|SetDirty (Actor|GetComponentbyClass (Components|GetOwner) "/Script/ConanSandbox.ConanBuildingPersistenceComponent") true 5.0))

(fn TrySendMessage
  (params (courier :type Game%20Item%20Object%20Reference) (payload :type Array%20of%20Game%20Item%20Object%20References) (recipientID :type String))
  (bind (_success _infomessage _pctweight) (CallFunction|ValidateMessage (Components|GetOwner) courier payload recipientID))
  (if _success
    (bind _templateid (Class|BPRACOICourier|GetBirdTemplateID(Message) courier))
    (LocalVariables|SetlocalCourierID _templateid)
    (bind (_accepted _errorinfo) (Default|MoveMessageIntoTransit (Utilities|GetMessagingSystem) (CallFunction|GetUniqueID) recipientID courier payload _pctweight))
    (Utilities|FlowControl|Sequence
      (:then_0
        (if _accepted
          (CallFunction|MulticastPlayBirdSound (LocalVariables|GetlocalCourierID))))
      (:then_1
        (return _accepted _errorinfo)))
    (else
      (return false _infomessage))))