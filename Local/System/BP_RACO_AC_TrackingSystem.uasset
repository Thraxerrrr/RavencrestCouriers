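; Tracking system component that keeps registries of trackable birds, nests, NPCs and player characters.
; Register and unregister functions validate the actor, then add it uniquely to or remove it from the list matching its category.
; A shared category macro identifies birds and nests by interface, then casts to ConanCharacter and uses IsPlayer to separate players from NPCs.
; Actors matching no category are not tracked, and the component runs no BeginPlay or Tick logic.
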(event EventBeginPlay)

(event EventTick
  (params (DeltaSeconds :type Float%20%28single-precision%29)))

(fn RegisterActor
  (params (actor :type Actor%20Object%20Reference))
  (bind _actor (LocalVariables|Getactor)
    (:then
      (Utilities|GetTrackingCategory _actor
        (:bird
          (Utilities|Array|AddUnique (Variables|Default|GettrackableBirds) actor))
        (:nest
          (Utilities|Array|AddUnique (Variables|Default|GettrackableNests) actor))
        (:NPC
          (Utilities|Array|AddUnique (Variables|Default|GettrackableNPCs) actor))
        (:playerCharacter
          (Utilities|Array|AddUnique (Variables|Default|GettrackablePlayers) actor))))
    (:else)))

(fn UnregisterActor
  (params (actor :type Actor%20Object%20Reference))
  (bind _actor (LocalVariables|Getactor)
    (:then
      (Utilities|GetTrackingCategory _actor
        (:bird
          (Utilities|Array|RemoveItem (Variables|Default|GettrackableBirds) actor))
        (:nest
          (Utilities|Array|RemoveItem (Variables|Default|GettrackableNests) actor))
        (:NPC
          (Utilities|Array|RemoveItem (Variables|Default|GettrackableNPCs) actor))
        (:playerCharacter
          (Utilities|Array|RemoveItem (Variables|Default|GettrackablePlayers) actor))))
    (:else)))