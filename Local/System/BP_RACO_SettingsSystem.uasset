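; Server settings actor for the RACO system, holding options for bird flights and XP, message checks, image rendering, detection mode, book copying and tracking.
; On BeginPlay the server assigns a persistence ID if none exists, registering it for database saving.
; UpdateServerSetting converts values by setting name, marks persistence dirty and prints the change.
; Getters expose each value, though GetIsNPCTrackingAllowed returns the player tracking flag.
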(event EventBeginPlay
  (if (Networking|IsServer)
    ;[1 1 1] Register for DB persistence
    (if (not (Class|DreamworldBlueprints|IsValidID (Class|PersistenceComponent|GetUniqueID (Variables|Default|GetActorPersistence))))
      (bind _returnvalue (Class|UniqueID|GenerateUniqueID))
      (Class|DreamworldBlueprints|SetUniqueID self _returnvalue)
      (Class|PersistenceComponent|SetDirty (Variables|Default|GetActorPersistence) true 5.0))))

(fn ConstructionScript)

(fn UpdateServerSetting
  (params (name :type String) (value :type String))
  (Utilities|FlowControl|Sequence
    (:then_0
      (switch string name
        (:Default
          (return))
        (:baseFlightDurationSec
          (Variables|RACO|serverSettings|SetbaseFlightDuration (Math|Conversions|ToInteger(Byte) value)))
        (:checkMessageFrequencySec
          (Variables|RACO|serverSettings|SetmeesageCheckFrequency (Math|Conversions|ToInteger(Byte) value)))
        (:allowRenderImages
          (Variables|RACO|serverSettings|SetisImageRenderingAllowed (CallFunction|ToBool value)))
        (:birdXPPerHour
          (Variables|RACO|serverSettings|SetbirdHourlyXP (Math|Conversions|ToInteger(Byte) value)))
        (:birdXPPerMessage
          (Variables|RACO|serverSettings|SetbirdTravelXP (Math|Conversions|ToInteger(Byte) value)))
        (:detectionModeEnabled
          (Variables|RACO|serverSettings|SetisDetectionModeAllowed (CallFunction|ToBool value)))
        (:allowCopyBooks
          (Variables|RACO|serverSettings|SetwhoCanCopyBooks (CallFunction|ToPlayerGroups value)))
        (:allowTracking
          (Variables|RACO|serverSettings|SetisTrackingAllowed (CallFunction|ToBool value)))
        (:allowNPCTracking
          (Variables|RACO|serverSettings|SetisNPCTrackingAllowed (CallFunction|ToBool value)))
        (:allowPlayerTracking
          (Variables|RACO|serverSettings|SetisPlayerTrackingAllowed (CallFunction|ToBool value)))))
    (:then_1
      (Class|PersistenceComponent|SetDirty (Variables|Default|GetActorPersistence) true 5.0)
      (Development|PrintString (Utilities|String|Append "Setting updated: " name " = " value) true true "(R=0.000000,G=0.660000,B=1.000000,A=1.000000)" 6.0)
      (return))))

(fn GetBaseFlightDuration
  (return (Variables|RACO|serverSettings|GetbaseFlightDuration)))

(fn GetMessageFrequencyCheck
  (return (Variables|RACO|serverSettings|GetmeesageCheckFrequency)))

(fn GetIsImageRenderingAllowed
  (return (Variables|RACO|serverSettings|GetisImageRenderingAllowed)))

(fn GetBirdHourlyXP
  (return (Variables|RACO|serverSettings|GetbirdHourlyXP)))

(fn GetBirdMessageXP
  (return (Variables|RACO|serverSettings|GetbirdTravelXP)))

(fn GetIsDetectionModeAllowed
  (return (Variables|RACO|serverSettings|GetisDetectionModeAllowed)))

(fn GetWhoCanCopyBooks
  (return (Variables|RACO|serverSettings|GetwhoCanCopyBooks)))

(fn GetIsTrackingAllowed
  (return (Variables|RACO|serverSettings|GetisTrackingAllowed)))

(fn GetIsNPCTrackingAllowed
  (return (Variables|RACO|serverSettings|GetisPlayerTrackingAllowed)))

(fn GetIsPlayerTrackingAllowed
  (return (Variables|RACO|serverSettings|GetisPlayerTrackingAllowed)))