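; Actor component that holds server settings for messenger birds, image rendering, detection mode, book copying and tracking permissions.
; UpdateServerSetting matches a setting by name, converts its value, marks the owner's PersistenceComponent dirty with a delay and prints the change; unknown names exit early.
; Getters expose each setting, though GetIsNPCTrackingAllowed returns the player tracking flag instead of the NPC one.
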(event EventBeginPlay)

(event EventTick
  (params (DeltaSeconds :type Float%20%28single-precision%29)))

(fn UpdateServerSetting
  (params (name :type String) (value :type String))
  (Utilities|FlowControl|Sequence
    (:then_0
      (switch string name
        (:Default
          (return))
        (:baseFlightDurationSec
          (Variables|Default|SetbaseFlightDuration (Math|Conversions|ToInteger(Byte) value)))
        (:allowRenderImages
          (Variables|Default|SetisImagesRenderingAllowed (CallFunction|ToBool value)))
        (:birdXPPerHour
          (Variables|Default|SetbirdHourlyXP (Math|Conversions|ToInteger(Byte) value)))
        (:birdXPPerMessage
          (Variables|Default|SetbirdTravelXP (Math|Conversions|ToInteger(Byte) value)))
        (:detectionModeEnabled
          (Variables|Default|SetisDetectionModeAllowed (CallFunction|ToBool value)))
        (:allowCopyBooks
          (Variables|Default|SetwhoCanCopyBooks (CallFunction|ToPlayerGroups value)))
        (:allowTracking
          (Variables|Default|SetisTrackingAllowed (CallFunction|ToBool value)))
        (:allowNPCTracking
          (Variables|Default|SetisNPCTrackingAllowed (CallFunction|ToBool value)))
        (:allowPlayerTracking
          (Variables|Default|SetisPlayerTrackingAllowed (CallFunction|ToBool value)))))
    (:then_1
      (Class|PersistenceComponent|SetDirty (Actor|GetComponentbyClass (Components|GetOwner) "/Script/UE4Dreamworld.PersistenceComponent") true 5.0)
      (Development|PrintString (Utilities|String|Append "Setting updated: " name " = " value) true true "(R=0.000000,G=0.660000,B=1.000000,A=1.000000)" 6.0)
      (return))))

(fn GetBaseFlightDuration
  (return (Variables|Default|GetbaseFlightDuration)))

(fn GetIsImageRenderingAllowed
  (return (Variables|Default|GetisImagesRenderingAllowed)))

(fn GetBirdHourlyXP
  (return (Variables|Default|GetbirdHourlyXP)))

(fn GetBirdMessageXP
  (return (Variables|Default|GetbirdTravelXP)))

(fn GetIsDetectionModeAllowed
  (return (Variables|Default|GetisDetectionModeAllowed)))

(fn GetWhoCanCopyBooks
  (return (Variables|Default|GetwhoCanCopyBooks)))

(fn GetIsTrackingAllowed
  (return (Variables|Default|GetisTrackingAllowed)))

(fn GetIsNPCTrackingAllowed
  (return (Variables|Default|GetisPlayerTrackingAllowed)))

(fn GetIsPlayerTrackingAllowed
  (return (Variables|Default|GetisPlayerTrackingAllowed)))