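; BP_RACO_A_Command is an actor that handles text commands for the RACO system, received with the calling player controller.
; Its DoCommand event branches on the first parameter: "set" passes a name and value to UpdateServerSetting on the RACO server settings.
; A "DownloadBook" check exists but does nothing, and a lookup of the player character component is left unconnected.
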(event EventDoCommand
  (params (Parameters :type Array%20of%20Strings) (CallingPlayerController :type Conan%20Player%20Controller%20Object%20Reference) (World :type World%20Object%20Reference))
  (bind _output (Utilities|Array|Get(acopy) Parameters))
  (if (Utilities|Enum|Equal(Enum) _output "set")
    (Default|UpdateServerSetting (CallFunction|GetServerSettingsRACO) (Utilities|Array|Get(acopy) Parameters 1) (Utilities|Array|Get(acopy) Parameters 2))
    (elif (Utilities|Enum|Equal(Enum) _output "DownloadBook")
      _)))

(fn ConstructionScript)