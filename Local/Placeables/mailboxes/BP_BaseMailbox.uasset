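; Base Blueprint for placeable mailboxes, with a crafting GUI center panel that depends on container access.
; Players with access get the mailbox inventory panel, while others get the deposit panel.
; On BeginPlay outside dedicated servers, non-brush instances hand their courier audio component to the messaging endpoint component.
; An interaction check can block riding characters and show them a HUD notification.
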(event EventBeginPlay
  (|CallParentFunction)
  (if (not (Variables|Default|GetIsABrush))
    (if (not (Networking|IsDedicatedServer))
      (Variables|/Game/Mods/RavencrestCouriers/System/BP_RACO_AC_MessagingEndpoint.BP_RACO_AC_MessagingEndpoint_C|SetaudioComponent (Variables|Default|GetBP_RACO_MessagingEndpoint_AC) (Variables|Default|GetCourierAudio)))))

(fn ConstructionScript
  (|CallParentFunction))

(fn InteractableActivateDisabled
  (params (InteractingCharacter :type Conan%20Character%20Object%20Reference))
  (return false))

(fn ClientGetCraftingGUICenterPanel
  (params (Instigator :type Player%20Controller%20Object%20Reference))
  (return (select (.CanAccess (Class|PlaceableBase|CanAccessContainer (Pawn|GetControlledPawn Instigator))) "MailboxInventory" "MailboxDeposit")))

(fn ShouldDisableInteraction
  (params (DisallowWhenMounted :type Boolean) (InteractingCharacter :type Conan%20Character%20Object%20Reference))
  (if (and (Class|ConanCharacter|IsRiding InteractingCharacter) DisallowWhenMounted)
    (bind _asconan_player_controller (Utilities|Casting|CastToConanPlayerController (Pawn|GetController InteractingCharacter))
      (:then
        (Class|ConanPlayerController|ClientHUDShowNotification _asconan_player_controller (Utilities|Text|MakeLiteralText "Cannot interact while riding") false true))
      (:CastFailed
        _))
    (return true)
    (else
      (return false))))