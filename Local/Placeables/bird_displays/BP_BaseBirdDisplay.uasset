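; Base placeable for bird displays, showing inventory bird items as animated meshes and optionally acting as a player proximity alarm.
; Inventory changes refresh matching mesh slots from bird type data, async-loading unloaded anim classes and offsetting from cached slot transforms.
; A persisted, server-applied config sizes the detection sphere and filters players by clan, playing the active bird's sound off dedicated servers with a five-second cooldown.
; Nesting functions are stubbed to refuse birds.
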(event SignalItemRemoved(PlaceableInventory)
  (params (index :type Integer) (item :type Game%20Item%20Object%20Reference) (dstInventory :type Item%20Inventory%20Object%20Reference) (dstIndex :type Integer))
  (CallFunction|RefreshBirdSlot 0 index))

(event OnComponentBeginOverlap(DetectionSphere)
  (params (OverlappedComponent :type Primitive%20Component%20Object%20Reference) (OtherActor :type Actor%20Object%20Reference) (OtherComp :type Primitive%20Component%20Object%20Reference) (OtherBodyIndex :type Integer) (bFromSweep :type Boolean) (SweepResult :type Hit%20Result%20Structure%20%28by%20ref%29))
  (CallFunction|HandleDetectionEvent OtherActor))

(event SignalItemAdded(PlaceableInventory)
  (params (index :type Integer) (item :type Game%20Item%20Object%20Reference) (srcInventory :type Item%20Inventory%20Object%20Reference) (srcIndex :type Integer))
  (CallFunction|RefreshBirdSlot item index))

(event Custom|asyncSetBirdSlotParameters
  (params (animClass :type AB%20Base%20Bird%20Soft%20Class%20Reference) (transform :type Transform) (birdSlot :type Skeletal%20Mesh%20Component%20Object%20Reference) (slotIndex :type Integer))
  (bind _class (Utilities|AsyncLoadClassAsset animClass)
    (:Completed
      (bind _asab_base_bird (Utilities|Casting|CastToAB_BaseBirdClass _class))
      (CallFunction|SetBirdSlotParameters _asab_base_bird transform birdSlot slotIndex))))

(event Custom|onTargetDetected
  (params (detectedActor :type Actor%20Object%20Reference) (activeBirdIndex :type Integer))
  (bind _placeableinventory (Variables|Default|GetPlaceableInventory))
  (bind _returnvalue (Class|ItemInventory|GetItem _placeableinventory activeBirdIndex))
  (if (not (Networking|IsDedicatedServer))
    (Utilities|IsValid _returnvalue
      (:Is%20Valid
        (bind _asbp_base_bird_item (Utilities|Casting|CastToBP_BaseBirdItem _returnvalue))
        (bind _typeid (Default|GetBirdType _asbp_base_bird_item))
        (CallFunction|PlayBirdSound (Variables|Default|GetBirdAudio) (CallFunction|GetBirdTypebyID _typeid))))))

(event Custom|onDataLoaded
  (EventDispatchers|UnbindEventfromOnSignalDataLoaded (Variables|Default|GetConanBuildingPersistence) (delegate Custom|onDataLoaded))
  (CallFunction|ApplyDetectionConfig))

(event EventBeginPlay
  (bind _conanbuildingpersistence (Variables|Default|GetConanBuildingPersistence))
  (|CallParentFunction)
  (if (not (Variables|Default|GetIsABrush))
    (Utilities|FlowControl|Sequence
      (:then_0
        (bind _array (CallFunction|GetBirdSlots))
        (bind (_array_element _array_index) (Utilities|ForEachLoopFast _array)
          (:LoopBody
            (Utilities|Array|SetArrayElem (Variables|Default|GetBirdSlotsTransforms) _array_index (Transformation|GetRelativeTransform _array_element) true))))
      (:then_1
        (if (Networking|IsServer)
          (Utilities|And+Branch (Variables|/Script/UE4Dreamworld.PersistenceComponent|Getm_bWasLoadedFromDB _conanbuildingpersistence) (not (Class|PersistenceComponent|IsDataDoneLoading _conanbuildingpersistence))
            (:True
              (EventDispatchers|BindEventtoOnSignalDataLoaded (Variables|Default|GetConanBuildingPersistence) (delegate Custom|onDataLoaded)))
            (:False
              (CallFunction|ApplyDetectionConfig)))
          (else
            (bind _returnvalue (Game|ConstructObjectfromClass "/Script/ConanSandbox.ItemInventoryClientMonitor"))
            (Class|ItemInventoryClientMonitor|SetInventory _returnvalue (Variables|Default|GetPlaceableInventory))))))))

(event EventCleanUp
  ;[1 1 1 0.3] Override the cleanup functionality so it does not remove Birdslots
)

(fn ConstructionScript
  (|CallParentFunction))

(fn GetBirdSlots
  (return (Utilities|Array|MakeArray (Variables|Default|GetBirdSlot01))))

(fn RefreshBirdSlot
  (params (item :type Game%20Item%20Object%20Reference) (slotIndex :type Integer))
  (bind _array (CallFunction|GetBirdSlots))
  (if (Utilities|Array|IsValidIndex _array slotIndex)
    (Utilities|IsValid item
      (:Is%20Valid
        (bind _asbp_base_bird_item (Utilities|Casting|CastToBP_BaseBirdItem item)
          (:then
            (bind _typeid (Default|GetBirdType _asbp_base_bird_item))
            (if (Utilities|IsValidClass (Utilities|ResolveSoftReference (.animClass (Utilities|Struct|BreakSTRUCT_RACO_BirdType (CallFunction|GetBirdTypebyID _typeid)))))
              (CallFunction|SetBirdSlotParameters (Utilities|ResolveSoftReference (.animClass (Utilities|Struct|BreakSTRUCT_RACO_BirdType (CallFunction|GetBirdTypebyID _typeid)))) (.transform (Utilities|Struct|BreakSTRUCT_RACO_BirdType (CallFunction|GetBirdTypebyID _typeid))) (Utilities|Array|Get(acopy) _array slotIndex) slotIndex)
              (else
                (CallFunction|AsyncSetBirdSlotParameters (.animClass (Utilities|Struct|BreakSTRUCT_RACO_BirdType (CallFunction|GetBirdTypebyID _typeid))) (.transform (Utilities|Struct|BreakSTRUCT_RACO_BirdType (CallFunction|GetBirdTypebyID _typeid))) (Utilities|Array|Get(acopy) _array slotIndex) slotIndex))))
          (:CastFailed
            (CallFunction|SetBirdSlotParameters :birdSlot (Utilities|Array|Get(acopy) _array slotIndex) :slotIndex slotIndex :!label _label))))
      (:Is%20Not%20Valid
        (goto _label)))))

(fn SetBirdSlotParameters
  (params (animClass :type AB%20Base%20Bird%20Class%20Reference) (transform :type Transform) (birdSlot :type Skeletal%20Mesh%20Component%20Object%20Reference) (slotIndex :type Integer))
  (bind _returnvalue (Class|DreamworldBlueprints|GetClassDefaultObject animClass))
  (bind _birdmesh (Default|GetBirdMesh _returnvalue))
  (if (Utilities|IsValidClass animClass)
    (Utilities|IsValid _birdmesh
      (:Is%20Valid
        (Components|SkinnedMesh|SetSkinnedAssetandUpdate birdSlot _birdmesh true)
        (Components|SkeletalMesh|SetAnimInstanceClass birdSlot animClass)
        (Transformation|SetRelativeTransform birdSlot (CallFunction|ApplyBirdTransform (Utilities|Array|Get(acopy) (Variables|Default|GetBirdSlotsTransforms) slotIndex) transform) false false)
        (Rendering|SetVisibility birdSlot true true))
      (:Is%20Not%20Valid
        (Rendering|SetVisibility birdSlot false true :!label _label)
        (Components|SkinnedMesh|SetSkinnedAssetandUpdate birdSlot 0 true)
        (Components|SkeletalMesh|SetAnimInstanceClass birdSlot 0)
        (Transformation|SetRelativeTransform birdSlot (Utilities|Array|Get(acopy) (Variables|Default|GetBirdSlotsTransforms) slotIndex) false false)))
    (else
      (goto _label))))

(fn RefreshAllSlots
  (bind _array (CallFunction|GetBirdSlots))
  (for (_ _array_index) _array
    (CallFunction|RefreshBirdSlot (Class|ItemInventory|GetItem (Variables|Default|GetPlaceableInventory) _array_index) _array_index)))

(fn HandleDetectionEvent
  (params (detectedActor :type Actor%20Object%20Reference))
  (bind _detectionconfig (Variables|Default|GetdetectionConfig))
  (bind (_activebirdindex _targets) (Utilities|Struct|BreakSTRUCT_RACO_BirdDetectionConfig _detectionconfig))
  (Utilities|And+Branch (Default|GetIsDetectionModeAllowed (CallFunction|GetServerSettingsRACO)) (!= -1 (.activeBirdIndex (Utilities|Struct|BreakSTRUCT_RACO_BirdDetectionConfig (Variables|Default|GetdetectionConfig))))
    (:True
      (if (>= (Math|DateTime|Now) (+ (Variables|Default|GetdetectionTime) (Math|Timespan|MakeTimespan 0 0 0 5)))
        (bind _asconan_character (Utilities|Casting|CastToConanCharacter detectedActor))
        (if (Class|ConanCharacter|IsPlayer _asconan_character)
          (switch Utilities|FlowControl|Switch|SwitchonENUM_RACO_BirdDetectionTargets _targets
            (:NewEnumerator0
              (if (Class|BuildableBase|IsOwner _asconan_character false)
                (CallFunction|OnTargetDetected detectedActor _activebirdindex :!label _label)
                (Variables|Default|SetdetectionTime (Math|DateTime|Now))))
            (:NewEnumerator1
              (if (not (Class|BuildableBase|IsOwner _asconan_character false))
                (goto _label)))
            (:NewEnumerator2
              (goto _label))))))))

(fn SetDetectionConfig
  (params (detectionConfig :type STRUCT%20RACO%20Bird%20Detection%20Config%20Structure))
  (if (Networking|IsServer)
    (Variables|Default|SetdetectionConfig detectionConfig)
    (Class|PersistenceComponent|SetDirty (Variables|Default|GetConanBuildingPersistence) true 5.0)
    (CallFunction|ApplyDetectionConfig)
    (return (Variables|/Script/Engine.PrimitiveComponent|GetbGenerateOverlapEvents (Variables|Default|GetDetectionSphere)))
    (else
      (return false))))

(fn GetDetectionConfig
  (return (Variables|Default|GetdetectionConfig)))

(fn ApplyDetectionConfig
  (bind _detectionconfig (Variables|Default|GetdetectionConfig))
  (bind _placeableinventory (Variables|Default|GetPlaceableInventory))
  (bind (_activebirdindex _radius) (Utilities|Struct|BreakSTRUCT_RACO_BirdDetectionConfig _detectionconfig))
  (bind _returnvalue (Class|ItemInventory|GetItem _placeableinventory _activebirdindex))
  (if (>= _activebirdindex 0)
    (Utilities|IsValid _returnvalue
      (:Is%20Valid
        (Utilities|Casting|CastToBP_BaseBirdItem _returnvalue
          (:then
            (Variables|/Script/Engine.PrimitiveComponent|SetbGenerateOverlapEvents (Variables|Default|GetDetectionSphere) (Default|GetIsDetectionModeAllowed (CallFunction|GetServerSettingsRACO)))
            (Components|Sphere|SetSphereRadius (Variables|Default|GetDetectionSphere) (Math|Conversions|ToFloat(Integer) _radius) true))
          (:CastFailed
            (Variables|/Script/Engine.PrimitiveComponent|SetbGenerateOverlapEvents (Variables|Default|GetDetectionSphere) false :!label _label))))
      (:Is%20Not%20Valid
        (goto _label)))
    (else
      (goto _label))))

(fn ClientGetCraftingGUICenterPanel
  (params (Instigator :type Player%20Controller%20Object%20Reference))
  (return "BirdDisplayInventory"))

(fn GetNestPopulation
  (return (Class|ItemInventory|GetItemList (Variables|Default|GetPlaceableInventory))))

(fn HasFreeNestingSlots
  (return false))

(fn NestFitsBird
  (params (bird :type Object%20Object%20Reference))
  (return false))

(fn TryNestBird
  (params (bird :type Game%20Item%20Object%20Reference))
  (return false ""))