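; BP_Coop_Medium2 is a medium coop placeable that provides twelve pet slots.
; Its CustomizePetSlots event gathers the slot references into the Pets array and resizes the idle animation, skeletal mesh and sound cue arrays to match that count.
; The construction script only calls the parent's, so the Blueprint's own logic is limited to this slot setup.
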(event EventCustomizePetSlots
  (bind _output_get (Variables|Default|SetPets (Utilities|Array|MakeArray (Variables|Default|GetPetSlot01) (Variables|Default|GetPetSlot02) (Variables|Default|GetPetSlot03) (Variables|Default|GetPetSlot04) (Variables|Default|GetPetSlot05) (Variables|Default|GetPetSlot06) (Variables|Default|GetPetSlot07) (Variables|Default|GetPetSlot08) (Variables|Default|GetPetSlot09) (Variables|Default|GetPetSlot10) (Variables|Default|GetPetSlot11) (Variables|Default|GetPetSlot12))))
  (bind _returnvalue (Utilities|Array|Length _output_get))
  (Utilities|Array|Resize (Variables|Default|GetPetIdleAnimations) _returnvalue)
  (Utilities|Array|Resize (Variables|Default|GetPetSkeletalMeshes) _returnvalue)
  (Utilities|Array|Resize (Variables|Default|GetPetSoundCues) _returnvalue))

(fn ConstructionScript
  (|CallParentFunction))