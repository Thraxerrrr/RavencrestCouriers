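; Base placeable bird coop that houses bird items in a pet inventory capped at MaxBirds, with a crafting GUI panel.
; Nesting helpers compare bird size to coop size, report free slots and move eligible birds into the inventory.
; Outside dedicated servers, inventory changes trigger a randomly delayed visual refresh.
; Each slot takes mesh and idle animation from the bird AnimClass's default object, offsets its cached transform (bats specially), or hides non-birds.
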(event Custom|HandlePetInventoryChanged
  (params (index :type Integer) (item :type Game%20Item%20Object%20Reference) (srcInventory :type Item%20Inventory%20Object%20Reference) (srcIndex :type Integer))
  ;[1 1 1 0.5] Handle bird animations
  (Utilities|FlowControl|Delay (Math|Random|RandomFloatinRange 0.0 1.0))
  (CallFunction|UpdateBirdAnimations))

(event Custom|HandlePetInventoryChanged2
  ;[1 1 1 0.5] Handle bird animations
  (Utilities|FlowControl|Delay (Math|Random|RandomFloatinRange 0.0 1.0))
  (CallFunction|UpdateBirdAnimations))

(event EventBeginPlay
  (|CallParentFunction)
  (if (not (Variables|Default|GetIsABrush))
    ;[1 1 1 0.5] Nest size
    (Class|ItemInventory|SetMaxItemCount (Variables|Default|GetPetInventory) (Variables|Default|GetmaxBirds))
    (if (not (Networking|IsDedicatedServer))
      (Utilities|FlowControl|Sequence
        (:then_0
          (Variables|/Game/Mods/RavencrestCouriers/System/BP_RACO_AC_MessagingEndpoint.BP_RACO_AC_MessagingEndpoint_C|SetaudioComponent (Variables|Default|GetBP_RACO_MessagingEndpoint_AC) (Variables|Default|GetCourierAudio))
          (Utilities|FlowControl|Delay 0.0)
          (CallFunction|CustomizePetSlots)
          (for (_array_element _array_index) (Variables|Default|GetPets)
            (Utilities|Array|SetArrayElem (Variables|Default|GetPetOriginalTransforms) _array_index (Transformation|GetRelativeTransform _array_element) true)))
        (:then_1
          ;[1 1 1 0.5] Handle bird animations
          (EventDispatchers|BindEventtoSignalItemAdded (Variables|Default|GetPetInventory) (delegate Custom|HandlePetInventoryChanged))
          (EventDispatchers|BindEventtoSignalItemRemoved (Variables|Default|GetPetInventory) (delegate Custom|HandlePetInventoryChanged))
          (EventDispatchers|BindEventtoSignalInventoryRecivedonClient (Variables|Default|GetPetInventory) (delegate Custom|HandlePetInventoryChanged2)))))))

(fn ConstructionScript
  (|CallParentFunction))

(fn CustomizePetSlots)

(fn ClientGetCraftingGUICenterPanel
  (params (Instigator :type Player%20Controller%20Object%20Reference))
  (return "BirdCoopInventory"))

(fn UpdateBirdAnimations
  (bind (_array_element _array_index) (Utilities|ForEachLoopFast (Variables|/Script/ConanSandbox.ItemInventory|GetItemList (Variables|Default|GetPetInventory)))
    (:LoopBody
      (LocalVariables|SetarrayIndex _array_index)
      (if (< (LocalVariables|GetarrayIndex) (Variables|Default|GetmaxBirds))
        (bind _asbp_base_bird_item (Utilities|Casting|CastToBP_BaseBirdItem _array_element)
          (:then
            (bind _birdtype (CallFunction|GetBirdTypebyID (Variables|/Game/Mods/RavencrestCouriers/Items/BP_BaseBirdItem.BP_BaseBirdItem_C|GetbirdTypeID _asbp_base_bird_item)))
            (bind _returnvalue (Class|FuncomGenericLibrary|SyncLoadClassAsset (.animClass (Utilities|Struct|BreakSTRUCT_RACO_BirdType _birdtype))))
            (Utilities|Array|SetArrayElem (Variables|Default|GetPetSkeletalMeshes) (LocalVariables|GetarrayIndex) (Default|GetBirdMesh (Class|DreamworldBlueprints|GetClassDefaultObject (.AsAB%20Base%20Bird (Utilities|Casting|CastToAB_BaseBirdClass _returnvalue)))) true)
            (Utilities|Array|SetArrayElem (Variables|Default|GetPetIdleAnimations) (LocalVariables|GetarrayIndex) (Default|GetIdleAnimation (Class|DreamworldBlueprints|GetClassDefaultObject (.AsAB%20Base%20Bird (Utilities|Casting|CastToAB_BaseBirdClass _returnvalue)))) true)
            (Transformation|SetRelativeTransform (Utilities|Array|Get(acopy) (Variables|Default|GetPets) (LocalVariables|GetarrayIndex)) (CallFunction|ApplyBirdTransform (Utilities|Array|Get(acopy) (Variables|Default|GetPetOriginalTransforms) (LocalVariables|GetarrayIndex)) (Math|Transform|ComposeTransforms (Math|Transform|SelectTransform (Variables|Default|GetbatTransform) (Math|Conversions|ToTransform(Vector) "0, 0, 0") (== (Variables|/Game/Mods/RavencrestCouriers/Items/BP_BaseBirdItem.BP_BaseBirdItem_C|GetbirdTypeID _asbp_base_bird_item) "bat")) (.transform (Utilities|Struct|BreakSTRUCT_RACO_BirdType _birdtype)))) false false))
          (:CastFailed
            (Utilities|Array|SetArrayElem (Variables|Default|GetPetSkeletalMeshes) (LocalVariables|GetarrayIndex) 0 true)
            (Utilities|Array|SetArrayElem (Variables|Default|GetPetIdleAnimations) (LocalVariables|GetarrayIndex) 0 true)
            (Transformation|SetRelativeScale3D (Utilities|Array|Get(acopy) (Variables|Default|GetPets) (LocalVariables|GetarrayIndex)) "0, 0, 0")))
        (else
          (CallFunction|SetPetVisuals :!label _label)
          (return))))
    (:Completed
      (goto _label))))

(fn GetNestPopulation
  (bind _array_element (Utilities|ForEachLoopFast (Variables|/Script/ConanSandbox.ItemInventory|GetItemList (Variables|Default|GetPetInventory)))
    (:LoopBody
      (Utilities|Array|Add (LocalVariables|GetnestedBirds) _array_element))
    (:Completed
      (return (LocalVariables|GetnestedBirds)))))

(fn HasFreeNestingSlots
  (return (< (Class|ItemInventory|GetPopulatedItemCount (Variables|Default|GetPetInventory) 0 -1) (Variables|Default|GetmaxBirds))))

(fn NestFitsBird
  (params (bird :type Object%20Object%20Reference))
  (bind _typeid (Class|BPRACOIBird|GetBirdType(Message) bird))
  (return (>= (CallFunction|MapBirdSizetoNumber (Variables|Default|Getsize)) (CallFunction|MapBirdSizetoNumber (.size (Utilities|Struct|BreakSTRUCT_RACO_BirdType (CallFunction|GetBirdTypebyID _typeid)))))))

(fn TryNestBird
  (params (bird :type Game%20Item%20Object%20Reference))
  (bind (_inventory _slot) (CallFunction|GetInventoryandSlot bird))
  (bind (_canenter _infomessage) (CallFunction|CanBirdEnterNest self bird))
  (if _canenter
    (bind _returnvalue (Class|ItemInventory|MoveItem _inventory _slot (Variables|Default|GetPetInventory) -1 -1 false))
    (return _returnvalue "")
    (else
      (return false _infomessage))))