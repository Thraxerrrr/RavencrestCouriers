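; BP_TestCoop is a test bird coop placeable that opens a bird coop crafting GUI when activated.
; Activation initializes the RACO messaging endpoint component, then ClientBindUI activates the GUI module with the returned destinations.
; GUI send requests go through the endpoint, binding a one-shot callback that returns acceptance or error feedback to the widget.
; Lock checks are still TODO, and unconnected test code adds backpack birds to PetInventory.
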(event Custom|ClientBindUI
  (params (destinations :type Array%20of%20STRUCT%20RACO%20Destination%20Structures))
  (bind _returnvalue (Class|GUIModuleController|ActivateModule (Class|GUIModuleController|GetGUIModuleController) (Utilities|Name|MakeLiteralName "RACO_BirdCoop_CraftingGUI") true false))
  (bind _asw_bird_coop_crafting_gui (Utilities|Casting|CastToW_BirdCoop_CraftingGUI _returnvalue))
  (EventDispatchers|BindEventtoSignalSendMessage _asw_bird_coop_crafting_gui (delegate Custom|OnSignalSendMessage))
  (Default|InitMessagingUI _asw_bird_coop_crafting_gui destinations))

(event Custom|OnSignalMessageSent
  (params (accepted :type Boolean) (errorMessage :type String) (messageRequest :type STRUCT%20RACO%20Message%20in%20Flight%20Structure))
  (EventDispatchers|UnbindEventfromSignalMessageSent (Variables|Default|GetBP_RACO_MessagingEndpoint_AC) (delegate Custom|OnSignalMessageSent))
  (Default|HandleMessageFeedback (stale Custom|ClientBindUI _asw_bird_coop_crafting_gui) accepted errorMessage messageRequest))

(event Custom|OnSignalSendMessage
  (params (carrier :type Game%20Item%20Ref%20Structure) (items :type Array%20of%20Game%20Item%20Ref%20Structures) (recipientID :type String))
  (bind _bp_raco_messagingendpoint_ac (Variables|Default|GetBP_RACO_MessagingEndpoint_AC))
  (EventDispatchers|BindEventtoSignalMessageSent _bp_raco_messagingendpoint_ac (delegate Custom|OnSignalMessageSent))
  (Default|TrySendMessage _bp_raco_messagingendpoint_ac carrier items recipientID))

(event EventInteractableActivate
  (params (Component :type Primitive%20Component%20Object%20Reference) (Instigator :type Player%20Controller%20Object%20Reference) (HitIndex :type Integer) (TriggeredFromRadialWheel :type Boolean))
  ;[1 1 1] TODO: add lock checks etc, see BP_Master_Placeables
  (Utilities|FlowControl|Sequence
    (:then_1
      (bind _destinations (Default|InitforMessagingUI (Variables|Default|GetBP_RACO_MessagingEndpoint_AC) Instigator (Utilities|Name|MakeLiteralName "RACO_BirdCoop_CraftingGUI")))
      (CallFunction|ClientBindUI _destinations))))

(fn ConstructionScript
  (|CallParentFunction))